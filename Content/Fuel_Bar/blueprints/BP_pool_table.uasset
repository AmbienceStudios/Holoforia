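; Pool table prop for the bar whose dressing is configured per instance in the construction script, with no runtime logic.
; Player 1 and Player 2 cue sticks are optional, each showing one of four preset positions chosen by its position setting.
; ReadyToPlay shows the racked balls and triangle; otherwise the script spawns the fifteen ball meshes at random spots and rotations on the table.
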(event EventBeginPlay)

(event Collision|EventActorBeginOverlap
  (params (OtherActor :type Actor%20Object%20Reference)))

(event EventTick
  (params (DeltaSeconds :type Float%20%28single-precision%29)))

(fn ConstructionScript
  (if (Variables|PoolTableRandomise|GetPlayer%201%20Stick)
    (Rendering|SetVisibility (Utilities|Array|Get(acopy) (Utilities|Array|MakeArray (Variables|Default|GetSM_pool_table_stick_01) (Variables|Default|GetSM_pool_table_stick_01_a) (Variables|Default|GetSM_pool_table_stick_01_b) (Variables|Default|GetSM_pool_table_stick_01_c)) (Variables|PoolTableRandomise|GetPlayer%201%20Stick%20Position)) true false))
  (if (Variables|PoolTableRandomise|GetPlayer%202%20Stick)
    (Rendering|SetVisibility (Utilities|Array|Get(acopy) (Utilities|Array|MakeArray (Variables|Default|GetSM_pool_table_stick_02) (Variables|Default|GetSM_pool_table_stick_02_a) (Variables|Default|GetSM_pool_table_stick_02_b) (Variables|Default|GetSM_pool_table_stick_02_c)) (Variables|PoolTableRandomise|GetPlayer%202%20Stick%20Position)) true false))
  (if (Variables|PoolTableRandomise|GetReady%20To%20Play)
    (Rendering|SetVisibility (Variables|Default|GetSM_pool_table_balls_07) true false)
    (else
      (for _index (range 0 14)
        (bind _returnvalue (AddComponent|AddStaticMeshComponent false (Math|Transform|MakeTransform (Math|Vector|MakeVector (Math|Random|RandomFloatinRange -105.0 105.0) (Math|Random|RandomFloatinRange -5e+01 5e+01) 86.599998) (Math|Random|RandomRotator false))))
        (Components|StaticMesh|SetStaticMesh _returnvalue (Utilities|Array|Get(acopy) (Utilities|Array|MakeArray "/Game/Fuel_Bar/mesh/SM_pool_table_balls_01.SM_pool_table_balls_01" "/Game/Fuel_Bar/mesh/SM_pool_table_balls_02.SM_pool_table_balls_02" "/Game/Fuel_Bar/mesh/SM_pool_table_balls_03.SM_pool_table_balls_03" "/Game/Fuel_Bar/mesh/SM_pool_table_balls_04.SM_pool_table_balls_04" "/Game/Fuel_Bar/mesh/SM_pool_table_balls_05.SM_pool_table_balls_05" "/Game/Fuel_Bar/mesh/SM_pool_table_balls_06.SM_pool_table_balls_06" "/Game/Fuel_Bar/mesh/SM_pool_table_balls_07.SM_pool_table_balls_07" "/Game/Fuel_Bar/mesh/SM_pool_table_balls_08.SM_pool_table_balls_08" "/Game/Fuel_Bar/mesh/SM_pool_table_balls_09.SM_pool_table_balls_09" "/Game/Fuel_Bar/mesh/SM_pool_table_balls_10.SM_pool_table_balls_10" "/Game/Fuel_Bar/mesh/SM_pool_table_balls_11.SM_pool_table_balls_11" "/Game/Fuel_Bar/mesh/SM_pool_table_balls_12.SM_pool_table_balls_12" "/Game/Fuel_Bar/mesh/SM_pool_table_balls_13.SM_pool_table_balls_13" "/Game/Fuel_Bar/mesh/SM_pool_table_balls_14.SM_pool_table_balls_14" "/Game/Fuel_Bar/mesh/SM_pool_table_balls_15.SM_pool_table_balls_15") _index))))))