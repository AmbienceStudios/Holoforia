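; Spline-driven prop Blueprint that lines up random liquor bottle meshes along an editable spline.
; The construction script steps along the spline length at fixed intervals, adding a static mesh component with a randomly picked bottle at each step.
; Each bottle follows the spline direction with slight sideways and yaw jitter, while its height is flattened to zero in local space.
; An older straight-line X-axis version remains unconnected, and the event graph is empty.
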(event EventBeginPlay)

(event Collision|EventActorBeginOverlap
  (params (OtherActor :type Actor%20Object%20Reference)))

(event EventTick
  (params (DeltaSeconds :type Float%20%28single-precision%29)))

(fn ConstructionScript
  (bind _spline (Variables|Default|GetSpline))
  (bind _spline_2 (Variables|Default|GetSpline))
  (for _index (range 0 (Math|Float|Floor (/ (Spline|GetDistanceAlongSplineatSplinePoint _spline_2 (- (Spline|GetNumberOfSplinePoints _spline_2) 1)) 1e+01)))
    (bind _returnvalue (AddComponent|AddStaticMeshComponent false (Math|Transform|MakeTransform (Math|Vector|MakeVector (.X (Math|Vector|BreakVector (Spline|GetLocationatDistanceAlongSpline _spline (* (Math|Conversions|ToFloat(Integer) _index) 1e+01) "Local"))) (+ (.Y (Math|Vector|BreakVector (Spline|GetLocationatDistanceAlongSpline _spline (* (Math|Conversions|ToFloat(Integer) _index) 1e+01) "Local"))) (Math|Random|RandomFloatinRange -2.0 2.0)) 0.0) (Math|Rotator|MakeRotator (.Roll (Math|Rotator|BreakRotator (Math|Conversions|RotationFromXVector (Math|Rotator|GetRotationXVector (Spline|GetRotationatDistanceAlongSpline _spline (* (Math|Conversions|ToFloat(Integer) _index) 1e+01) "Local"))))) (.Pitch (Math|Rotator|BreakRotator (Math|Conversions|RotationFromXVector (Math|Rotator|GetRotationXVector (Spline|GetRotationatDistanceAlongSpline _spline (* (Math|Conversions|ToFloat(Integer) _index) 1e+01) "Local"))))) (+ (.Yaw (Math|Rotator|BreakRotator (Math|Conversions|RotationFromXVector (Math|Rotator|GetRotationXVector (Spline|GetRotationatDistanceAlongSpline _spline (* (Math|Conversions|ToFloat(Integer) _index) 1e+01) "Local"))))) (Math|Random|RandomFloatinRange -1e+01 1e+01))))))
    (Components|StaticMesh|SetStaticMesh _returnvalue (Utilities|Array|Get(acopy) (Utilities|Array|MakeArray "/Game/Fuel_Bar/mesh/SM_small_props_liquor_bottle_01.SM_small_props_liquor_bottle_01" "/Game/Fuel_Bar/mesh/SM_small_props_liquor_bottle_02.SM_small_props_liquor_bottle_02" "/Game/Fuel_Bar/mesh/SM_small_props_liquor_bottle_03.SM_small_props_liquor_bottle_03" "/Game/Fuel_Bar/mesh/SM_small_props_liquor_bottle_05.SM_small_props_liquor_bottle_05" "/Game/Fuel_Bar/mesh/SM_small_props_liquor_bottle_06.SM_small_props_liquor_bottle_06" "/Game/Fuel_Bar/mesh/SM_small_props_liquor_bottle_07.SM_small_props_liquor_bottle_07" "/Game/Fuel_Bar/mesh/SM_small_props_liquor_bottle_08.SM_small_props_liquor_bottle_08" "/Game/Fuel_Bar/mesh/SM_small_props_liquor_bottle_09.SM_small_props_liquor_bottle_09" "/Game/Fuel_Bar/mesh/SM_small_props_liquor_bottle_10.SM_small_props_liquor_bottle_10" "/Game/Fuel_Bar/mesh/SM_small_props_liquor_bottle_04.SM_small_props_liquor_bottle_04") (Math|Random|RandomInteger 10)))))