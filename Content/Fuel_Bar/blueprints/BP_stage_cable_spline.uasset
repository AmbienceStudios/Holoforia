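; Spline-driven cable actor, apparently for stage dressing, that builds its meshes in the construction script and has no active event logic.
; Each pair of neighboring spline points gets a spline mesh segment shaped by their local positions and tangents.
; StartSocket and EndSocket flags add static meshes at the spline ends, the end one rotated 180 degrees.
; These socket checks sit inside the segment loop, so socket meshes repeat per segment.
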(event EventBeginPlay)

(event Collision|EventActorBeginOverlap
  (params (OtherActor :type Actor%20Object%20Reference)))

(event EventTick
  (params (DeltaSeconds :type Float%20%28single-precision%29)))

(fn ConstructionScript
  (bind _spline (Variables|Default|GetSpline))
  (bind _spline_2 (Variables|Default|GetSpline))
  (bind _returnvalue (Spline|GetNumberOfSplinePoints _spline_2))
  (for _index (range 0 (- (Spline|GetNumberOfSplinePoints (Variables|Default|GetSpline)) 2))
    (bind _returnvalue_2 (AddComponent|AddSplineMeshComponent false))
    (Transformation|AttachComponentToComponent _returnvalue_2 (Variables|Default|GetDefaultSceneRoot) "None" "KeepRelative" "KeepRelative" "KeepRelative" true)
    (SplineMesh|SetStartandEnd _returnvalue_2 (.Location (Spline|GetLocationandTangentatSplinePoint _spline _index "Local")) (.Tangent (Spline|GetLocationandTangentatSplinePoint _spline _index "Local")) (.Location (Spline|GetLocationandTangentatSplinePoint _spline (+ _index 1) "Local")) (.Tangent (Spline|GetLocationandTangentatSplinePoint _spline (+ _index 1) "Local")) true :!class /Script/Engine.SplineMeshComponent)
    (if (Variables|Default|GetStart%20Socket)
      (AddComponent|AddStaticMeshComponent false (Math|Transform|MakeTransform (Spline|GetLocationatSplinePoint _spline_2 0 "Local") (Spline|GetRotationatSplinePoint _spline_2 0 "World"))))
    (if (Variables|Default|GetEnd%20Socket)
      (bind _returnvalue_3 (AddComponent|AddStaticMeshComponent false (Math|Transform|MakeTransform (Spline|GetLocationatSplinePoint _spline_2 _returnvalue "Local") (Spline|GetRotationatSplinePoint _spline_2 _returnvalue "World"))))
      (Transformation|AddLocalRotation _returnvalue_3 "0,180.000000, 0" false false))))