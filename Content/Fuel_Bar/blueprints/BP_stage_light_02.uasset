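; Configurable stage spotlight prop built entirely in the construction script, with no active runtime logic.
; LightColor drives both the head's emissive material parameter and the SpotLight color, while ArmRotation yaws the arm and HeadRotation pitches the head.
; A spline point snaps to the Cube component's world location, then a spline mesh component is generated for each segment between consecutive points.
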(event EventBeginPlay)

(event Collision|EventActorBeginOverlap
  (params (OtherActor :type Actor%20Object%20Reference)))

(event EventTick
  (params (DeltaSeconds :type Float%20%28single-precision%29)))

(fn ConstructionScript
  (bind _spline (Variables|Default|GetSpline))
  (bind _light_color (Variables|StageLight|GetLight%20Color))
  (Rendering|Material|SetVectorParameterValueonMaterials (Variables|Default|GetSM_Light_stage_02_head) "Emissive Color" (Math|Conversions|ToVector(LinearColor) _light_color))
  (Rendering|Components|Light|SetLightColor (Variables|Default|GetSpotLight) _light_color true)
  (Transformation|AddLocalRotation (Variables|Default|GetSM_Light_stage_02_arm) (Math|Rotator|MakeRotator 0.0 0.0 (Variables|StageLight|GetArm%20Rotation)) false false)
  (Transformation|AddLocalRotation (Variables|Default|GetSM_Light_stage_02_head) (Math|Rotator|MakeRotator 0.0 (Variables|StageLight|GetHead%20Rotation) 0.0) false false)
  (Spline|SetLocationatSplinePoint (Variables|Default|GetSpline) 0 (Transformation|GetWorldLocation (Variables|Default|GetCube)) "World" true)
  (for _index (range 0 (- (Spline|GetNumberOfSplinePoints (Variables|Default|GetSpline)) 2))
    (bind _returnvalue (AddComponent|AddSplineMeshComponent false))
    (Transformation|AttachComponentToComponent _returnvalue (Variables|Default|GetDefaultSceneRoot) "None" "KeepRelative" "KeepRelative" "KeepRelative" true)
    (SplineMesh|SetStartandEnd _returnvalue (.Location (Spline|GetLocationandTangentatSplinePoint _spline _index "Local")) (.Tangent (Spline|GetLocationandTangentatSplinePoint _spline _index "Local")) (.Location (Spline|GetLocationandTangentatSplinePoint _spline (+ _index 1) "Local")) (.Tangent (Spline|GetLocationandTangentatSplinePoint _spline (+ _index 1) "Local")) true :!class /Script/Engine.SplineMeshComponent)))