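; BP_stage_light_01 is a configurable stage light prop with an arm mesh, a head mesh and a spotlight.
; The construction script applies LightColor to both the spotlight and the head material's "Emissive Color" parameter, keeping glow and light matched.
; It adds ArmRotation as local yaw on the arm and HeadRotation as local pitch on the head to aim the fixture.
; The event graph holds no runtime logic.
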(event EventBeginPlay)

(event Collision|EventActorBeginOverlap
  (params (OtherActor :type Actor%20Object%20Reference)))

(event EventTick
  (params (DeltaSeconds :type Float%20%28single-precision%29)))

(fn ConstructionScript
  (bind _light_color (Variables|StageLight|GetLight%20Color))
  (Rendering|Material|SetVectorParameterValueonMaterials (Variables|Default|GetSM_Light_stage_01_head) "Emissive Color" (Math|Conversions|ToVector(LinearColor) _light_color))
  (Rendering|Components|Light|SetLightColor (Variables|Default|GetSpotLight) _light_color true)
  (Transformation|AddLocalRotation (Variables|Default|GetSM_Light_stage_01_arm) (Math|Rotator|MakeRotator 0.0 0.0 (Variables|StageLight|GetArm%20Rotation)) false false)
  (Transformation|AddLocalRotation (Variables|Default|GetSM_Light_stage_01_head) (Math|Rotator|MakeRotator 0.0 (Variables|StageLight|GetHead%20Rotation) 0.0) false false))