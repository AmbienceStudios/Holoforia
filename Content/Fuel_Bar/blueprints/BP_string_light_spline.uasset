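; Spline-driven string light prop that builds a strand of lamps along an editable spline in the construction script.
; Lamp static meshes are spawned at even intervals, with LampDensity setting the approximate spacing, each oriented along the spline with a slight offset.
; A spline mesh component is then stretched between each pair of spline points, following their tangents, to form the connecting strand.
; The event graph holds no runtime logic.
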(event EventBeginPlay)

(event Collision|EventActorBeginOverlap
  (params (OtherActor :type Actor%20Object%20Reference)))

(event EventTick
  (params (DeltaSeconds :type Float%20%28single-precision%29)))

(fn ConstructionScript
  (bind _lamp_density (Variables|StringLight|GetLamp%20Density))
  (bind _spline (Variables|Default|GetSpline))
  (bind _spline_2 (Variables|Default|GetSpline))
  (bind _returnvalue (Spline|GetNumberOfSplinePoints _spline_2))
  (bind _returnvalue_2 (- _returnvalue 1))
  (bind _returnvalue_3 (Spline|GetDistanceAlongSplineatSplinePoint _spline_2 _returnvalue_2))
  (bind _returnvalue_4 (/ _returnvalue_3 _lamp_density))
  (bind _returnvalue_5 (Math|Float|Truncate _returnvalue_4))
  (for _index (range 0 (- _returnvalue_5 1))
    (bind _returnvalue_6 (AddComponent|AddStaticMeshComponent false (Math|Transform|MakeTransform (Math|Vector|MakeVector (.X (Math|Vector|BreakVector (Spline|GetLocationatDistanceAlongSpline _spline (* _index (/ _returnvalue_3 (Math|Conversions|ToFloat(Integer) _returnvalue_5))) "Local"))) (- (.Y (Math|Vector|BreakVector (Spline|GetLocationatDistanceAlongSpline _spline (* _index (/ _returnvalue_3 (Math|Conversions|ToFloat(Integer) _returnvalue_5))) "Local"))) 0.15) (+ (.Z (Math|Vector|BreakVector (Spline|GetLocationatDistanceAlongSpline _spline (* _index (/ _returnvalue_3 (Math|Conversions|ToFloat(Integer) _returnvalue_5))) "Local"))) 0.5)) (Math|Conversions|RotationFromXVector (Math|Rotator|GetRotationXVector (Spline|GetRotationatDistanceAlongSpline _spline (* _index (/ _returnvalue_3 (Math|Conversions|ToFloat(Integer) _returnvalue_5))) "Local"))))))
    (Components|StaticMesh|SetStaticMesh _returnvalue_6 (Utilities|Array|Get(acopy) (Utilities|Array|MakeArray "/Game/Fuel_Bar/mesh/SM_Light_string_lamp.SM_Light_string_lamp") (Math|Random|RandomInteger 1))))
  (for _index_2 (range 0 (- (Spline|GetNumberOfSplinePoints (Variables|Default|GetSpline)) 2))
    (bind _returnvalue_7 (AddComponent|AddSplineMeshComponent false))
    (Transformation|AttachComponentToComponent _returnvalue_7 (Variables|Default|GetSpline) "None" "KeepRelative" "KeepRelative" "KeepRelative" true)
    (SplineMesh|SetStartandEnd _returnvalue_7 (.Location (Spline|GetLocationandTangentatSplinePoint (Variables|Default|GetSpline) _index_2 "Local")) (.Tangent (Spline|GetLocationandTangentatSplinePoint (Variables|Default|GetSpline) _index_2 "Local")) (.Location (Spline|GetLocationandTangentatSplinePoint (Variables|Default|GetSpline) (+ _index_2 1) "Local")) (.Tangent (Spline|GetLocationandTangentatSplinePoint (Variables|Default|GetSpline) (+ _index_2 1) "Local")) true :!class /Script/Engine.SplineMeshComponent)))