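; BP_NPC_WayPoint is a waypoint marker in the NPC Manager's navigation assets, identified by a group name and a numeric ID.
; Its construction script writes both values to text components and applies flags for text visibility, sphere visibility and hiding the sphere in game.
; FnSetWayPointInfo repeats only the text update, so the labels can be refreshed separately from construction.
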(fn ConstructionScript
  ;[1 1 1] Set text
  (Rendering|Components|TextRender|SetText (Variables|Default|GetPathName) (Variables|Setup|GetWayPointGroupName))
  (Rendering|Components|TextRender|SetText (Variables|Default|GetID) (Utilities|Text|ToText(Integer) (Variables|Setup|GetWayPointID)))
  ;[1 1 1] Set visibility
  (Rendering|SetVisibility (Variables|Default|GetPathName) (Variables|Setup|GetTextVisible) true)
  (Rendering|SetVisibility (Variables|Default|GetSphere) (Variables|Setup|GetMarkerVisible) false)
  (Development|SetHiddeninGame (Variables|Default|GetSphere) (Variables|Setup|GetMarkerHidden) false))

(fn FnSetWayPointInfo
  (Rendering|Components|TextRender|SetText (Variables|Default|GetPathName) (Variables|Setup|GetWayPointGroupName))
  (Rendering|Components|TextRender|SetText (Variables|Default|GetID) (Utilities|Text|ToText(Integer) (Variables|Setup|GetWayPointID))))