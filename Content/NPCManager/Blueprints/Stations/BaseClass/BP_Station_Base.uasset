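; Base NPC station actor: a placeable spot that notifies arriving NPCs and supplies its station info.
; BeginPlay stores the Arrow transform in the station options; trigger overlap messages the actor's Comp_NPC_Controller through a DoOnce, reset on exit.
; The construction script configures area, nav blocker, prop and preview pose, colouring the area by Regular, Linked or Sequence type.
; Helpers expose entry point, linked-station readiness, prop visibility and interact messages to listed actors.
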(event OnComponentBeginOverlap(Trigger)
  (params (OverlappedComponent :type Primitive%20Component%20Object%20Reference) (OtherActor :type Actor%20Object%20Reference) (OtherComp :type Primitive%20Component%20Object%20Reference) (OtherBodyIndex :type Integer) (bFromSweep :type Boolean) (SweepResult :type Hit%20Result%20Structure%20%28by%20ref%29))
  (Variables|Default|SetOverlappedActor OtherActor)
  ;[1 1 1] Check actor implements the NPC Controller BPI
  (Utilities|IsValid (Actor|GetComponentbyClass (Variables|Default|GetOverlappedActor) "/Game/NPCManager/Blueprints/Characters/NPC/Comp_NPC_Controller.Comp_NPC_Controller_C")
    (:Is%20Valid
      (Variables|Default|SetNPC_Controller (Actor|GetComponentbyClass (Variables|Default|GetOverlappedActor) "/Game/NPCManager/Blueprints/Characters/NPC/Comp_NPC_Controller.Comp_NPC_Controller_C"))
      (Utilities|FlowControl|DoOnce false
        (:Completed
          ;[1 1 1] Send Message - Arrived at Station
          (Class|BPINPCController|FnArrivedatStation(Message) (Variables|Default|GetNPC_Controller) self (Variables|Setup|GetStationOptions)))))))

(event OnComponentEndOverlap(Trigger)
  (params (OverlappedComponent :type Primitive%20Component%20Object%20Reference) (OtherActor :type Actor%20Object%20Reference) (OtherComp :type Primitive%20Component%20Object%20Reference) (OtherBodyIndex :type Integer))
  (Variables|Default|SetOverlappedActor OtherActor)
  ;[1 1 1] Check actor implements the NPC Controller BPI
  (Utilities|IsValid (Actor|GetComponentbyClass (Variables|Default|GetOverlappedActor) "/Game/NPCManager/Blueprints/Characters/NPC/Comp_NPC_Controller.Comp_NPC_Controller_C")
    (:Is%20Valid
      (Variables|Default|SetNPC_Controller (Actor|GetComponentbyClass (Variables|Default|GetOverlappedActor) "/Game/NPCManager/Blueprints/Characters/NPC/Comp_NPC_Controller.Comp_NPC_Controller_C"))
      (Utilities|FlowControl|DoOnce false) ; enters at Reset
    )))

(event EventBeginPlay
  (bind _arrow (Variables|Default|GetArrow))
  (bind _returnvalue (Transformation|GetWorldTransform _arrow))
  ;[1 1 1] Set Station Transform
  (Utilities|Struct|SetmembersinStruct_NPC_StationInfo (Variables|Setup|GetStationOptions) (Math|Transform|MakeTransform (.location _returnvalue) (.rotation _returnvalue))))

(fn ConstructionScript
  (bind _generalsettings (Variables|Setup|GetGeneralSettings))
  (bind _generalsettings_2 (Variables|Setup|GetGeneralSettings))
  (bind _generalsettings_3 (Variables|Setup|GetGeneralSettings))
  (bind _generalsettings_4 (Variables|Setup|GetGeneralSettings))
  (bind (_posemesh _posematerial) (Utilities|Struct|BreakStruct_Station_GeneralOptions _generalsettings))
  (bind (_areascale _navmeshvolumescale) (Utilities|Struct|BreakStruct_Station_GeneralOptions _generalsettings_2))
  (bind (_areavisible _areahidden _posehidden) (Utilities|Struct|BreakStruct_Station_GeneralOptions _generalsettings_3))
  (bind (_propmesh _posemesh_2) (Utilities|Struct|BreakStruct_Station_GeneralOptions _generalsettings_4))
  ;[1 1 1] Set area scale and Nav Mesh Blocker box extent
  (Transformation|SetWorldScale3D (Variables|Default|GetArea) _areascale)
  (Transformation|SetWorldScale3D (Variables|Default|GetNavMeshBlocker) _navmeshvolumescale)
  ;[1 1 1] Set Area visibility
  (Rendering|SetVisibility (Variables|Default|GetArea) _areavisible false)
  (Development|SetHiddeninGame (Variables|Default|GetArea) _areahidden false)
  (Development|SetHiddeninGame (Variables|Default|GetPoseSkeleton) _posehidden false)
  ;[1 1 1] Set the Station Type
  (CallFunction|FnSetStationType)
  ;[1 1 1] Set Prop and Pose meshes
  (Components|StaticMesh|SetStaticMesh (Variables|Default|GetProp) _propmesh)
  (Class|SkinnedMeshComponent|SetSkeletalMesh (Variables|Default|GetPoseSkeleton) _posemesh_2 true)
  ;[1 1 1] Set pose mesh materials
  (for (_ _array_index) (Variables|/Script/Engine.SkeletalMesh|GetMaterials _posemesh)
    (Rendering|Material|SetMaterial (Variables|Default|GetPoseSkeleton) _array_index _posematerial)))

(fn FnGetEntryPoint
  ;[1 1 1] Return the entry point as the location of the Arrow component
  (return (Transformation|GetWorldLocation (Variables|Default|GetArrow))))

(fn FnSetStationType
  ;[1 1 1] Switch on Station Type
  (switch Utilities|FlowControl|Switch|SwitchonEnum_StationType (.StationType (Utilities|Struct|BreakStruct_NPC_StationInfo (Variables|Setup|GetStationOptions)))
    (:NewEnumerator0
      ;[1 1 1] Set the material based on the type
      (Rendering|Material|SetMaterial (Variables|Default|GetArea) 0 "/Game/NPCManager/Materials/Translucent/M_Translucent_Purple.M_Translucent_Purple"))
    (:NewEnumerator1
      (Rendering|Material|SetMaterial (Variables|Default|GetArea) 0 "/Game/NPCManager/Materials/Translucent/M_Translucent_Blue.M_Translucent_Blue"))
    (:NewEnumerator2
      (Rendering|Material|SetMaterial (Variables|Default|GetArea) 0 "/Game/NPCManager/Materials/Translucent/M_Translucent_Green.M_Translucent_Green"))))

(fn FnCheckLinkedStations
  (bind _array_element (Utilities|Array|ForEachLoopwithBreak (Variables|Setup|GetLinkedStations) :!label _label)
    (:LoopBody
      (bind _output_get (LocalVariables|SetStation _array_element))
      (if (Variables|BP_Station_Base_C|GetStationLinked _output_get)
        (LocalVariables|SetAllLinked true)
        (else
          (LocalVariables|SetAllLinked false)
          (goto _label Break))))
    (:Completed
      (return (LocalVariables|GetAllLinked)))))

(fn FnShowHideProp
  (params (Show :type Boolean))
  (Rendering|SetVisibility (Variables|Default|GetProp) Show false))

(event Custom|EventUseInteractions
  ;[1 1 1] Do we want to interact with other objects?
  (if (Utilities|Struct|BreakStruct_Station_InteractionOptions (Variables|Setup|GetInteractionOptions))
    ;[1 1 1] Loop through list of actors and send Interact message
    (for _array_element (Utilities|Struct|BreakStruct_Station_InteractionOptions (Variables|Setup|GetInteractionOptions))
      (Class|BPINPCInteraction|FnInteract(Message) _array_element (Variables|Default|GetOverlappedActor)))))