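; Server-authoritative manager that registers NPCs, maps level POIs, caches tagged players and checks for nav mesh bounds.
; A looping timer sorts NPCs into active, partial or inactive by 2D distance to the nearest player and pushes that state to each Comp_NPC_Controller.
; Hour updates fire new-hour and day start/end dispatchers.
; Optional debug aids print proximity and render stats, draw radius traces and apply global time dilation.
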(event Custom|EventCheckForPlayers
  (bind _returnvalue (Utilities|Time|SetTimerbyEvent (delegate Custom|EventCheckForPlayers) (Variables|Setup-Proximity|GetProximityCheckFreq) true))
  (Variables|Default|SetProximityHandler _returnvalue)
  ;[1 1 1] Set the NPCs Proximity State
  (CallFunction|FnSetNPCProximityState)
  ;[1 1 1] Show Activation Stats
  (if (Variables|Setup-Proximity|GetShowActivationStats)
    (Networking|SwitchHasAuthority
      (:Authority
        (|PRINTREPORT)))))

(event Custom|EventCheckNPCRendering
  (Utilities|Time|SetTimerbyEvent (delegate Custom|EventCheckNPCRendering) (Variables|Default|GetCheckRenderFreq) true)
  (CallFunction|FnShowRenderStas))

(event Custom|Set%20Time%20Dilation
  (Utilities|Time|SetGlobalTimeDilation (Variables|Setup|GetTimeDilation)))

(event EventBeginPlay
  (Networking|SwitchHasAuthority
    (:Authority
      (CallFunction|FnGetAllPOIs)
      (CallFunction|FnCheckLevel)
      (Utilities|FlowControl|Sequence
        (:then_0
          (Utilities|FlowControl|Delay 1.0)
          (CallFunction|FnGetPlayers))
        (:then_1
          (if (Variables|Setup-Proximity|GetUseProximitySystem)
            (CallFunction|EventCheckforPlayers)))
        (:then_2
          (if (Variables|Setup|GetShowRenderStas)
            (CallFunction|EventCheckNPCRendering)))
        (:then_3
          (if (Variables|Setup|GetUseTimeDilation)
            (Utilities|Time|SetGlobalTimeDilation (Variables|Setup|GetTimeDilation))))))))

(fn ConstructionScript)

(fn FnRegisterNPC
  (params (NPC :type Actor%20Object%20Reference))
  (Utilities|Array|Add (Variables|Setup|GetNPCList) NPC))

(fn FnGetAllPOIs
  ;[1 1 1] Clear the POI Map
  (Utilities|Map|Clear (Variables|Setup|GetPOIMap))
  ;[1 1 1] Go through all POIs in the scene
  (bind _outactors (Actor|GetAllActorsOfClass "/Game/NPCManager/Blueprints/POIs/BaseClasses/BP_NPC_POI_Base.BP_NPC_POI_Base_C"))
  (for _array_element _outactors
    (LocalVariables|SetPOI _array_element)
    ;[1 1 1] Add the POI to the map
    (Utilities|Map|Add (Variables|Setup|GetPOIMap) (Utilities|GetClass (LocalVariables|GetPOI)) (LocalVariables|GetPOI))
    ;[1 1 1] Set Self as POI's NPC Manager
    (Variables|/Game/NPCManager/Blueprints/POIs/BaseClasses/BP_NPC_POI_Base.BP_NPC_POI_Base_C|SetNPCManager (LocalVariables|GetPOI) self)))

(fn FnGetTimeOfDay
  (Utilities|IsValid (Variables|Setup|GetDayCycleBP)
    (:Is%20Valid
      (return true (Variables|TOD|GetCurrentHour)))
    (:Is%20Not%20Valid
      (return false 0.0))))

(fn FnCheckLevel
  (Utilities|FlowControl|Sequence
    (:then_0
      ;[1 1 1] Check for a Nav Mesh in the level
      (bind _outactors (Actor|GetAllActorsOfClass "/Script/NavigationSystem.NavMeshBoundsVolume"))
      (if (Utilities|Array|IsValidIndex _outactors)
        (LocalVariables|SetFoundNavMesh true)
        (else
          (LocalVariables|SetFoundNavMesh false))))
    (:then_1
      (|REPORT))))

(fn FnGetPlayers
  (Utilities|FlowControl|Sequence
    (:then_0
      ;[1 1 1] Get all actors with the Player Tag
      (bind _outactors (Actor|GetAllActorswithTag "Player"))
      (Variables|Setup-Proximity|SetPlayerList _outactors))
    (:then_1
      ;[1 1 1] Populate the Player Names and IDs arrays
      (for _array_element (Variables|/Script/Engine.GameStateBase|GetPlayerArray (Game|GetGameState))
        (Utilities|Array|Add (Variables|Setup-Proximity|GetPlayerNames) (PlayerState|GetPlayerName _array_element))
        (Utilities|Array|Add (Variables|Setup-Proximity|GetPlayerIDs) (Variables|/Script/Engine.PlayerState|GetPlayerId _array_element))))))

(fn FnSetNPCProximityState
  ;[1 1 1] Clear lists
  (Utilities|Array|Clear (Variables|Setup|GetActiveNPCs))
  (Utilities|Array|Clear (Variables|Setup|GetPartialActiveNPCs))
  (Utilities|Array|Clear (Variables|Setup|GetInactiveNPCs))
  ;[1 1 1] Go through all NPCs in the level
  (for _array_element (Variables|Setup|GetNPCList)
    (bind _output_get (LocalVariables|SetNPC _array_element))
    (Utilities|IsValid _output_get
      (:Is%20Valid
        ;[1 1 1] Loop through all Players
        (for _array_element_2 (Variables|Setup-Proximity|GetPlayerList)
          (LocalVariables|SetPlayer _array_element_2)
          (Utilities|FlowControl|Sequence
            (:then_0
              ;[1 1 1] Calculate the NPC distance to the Player
              (Utilities|Array|Add (LocalVariables|GetDistanceList) (Math|Vector|Distance2D(Vector) (Transformation|GetActorLocation (LocalVariables|GetNPC)) (Transformation|GetActorLocation (LocalVariables|GetPlayer)))))
            (:then_1
              (|SHOWTRACES))))
        ;[1 1 1] Get distance to closest Player
        (LocalVariables|SetNPCDistance (.MinValue (Math|Float|MinOfFloatArray (LocalVariables|GetDistanceList))))
        ;[1 1 1] Is the NPC farther than the Partial Activation Radius?
        (if (> (LocalVariables|GetNPCDistance) (Variables|Setup-Proximity|GetPartialActivationRadius))
          ;[1 1 1] Add to Inactive list
          (Utilities|Array|Add (Variables|Setup|GetInactiveNPCs) (LocalVariables|GetNPC))
          (else
            ;[1 1 1] Is the NPC farther than the Full Activation Radius?
            (if (> (LocalVariables|GetNPCDistance) (Variables|Setup-Proximity|GetFullActivationRadius))
              ;[1 1 1] Add to Partial Active List
              (Utilities|Array|Add (Variables|Setup|GetPartialActiveNPCs) (LocalVariables|GetNPC))
              (else
                ;[1 1 1] Add to Active List
                (Utilities|Array|Add (Variables|Setup|GetActiveNPCs) (LocalVariables|GetNPC)))))))))
  (Utilities|FlowControl|Sequence
    (:then_0
      ;[1 1 1] Activate the NPCs
      (for _array_element_3 (Variables|Setup|GetActiveNPCs)
        (Utilities|IsValid _array_element_3
          (:Is%20Valid
            (Variables|/Game/NPCManager/Blueprints/Characters/NPC/Comp_NPC_Controller.Comp_NPC_Controller_C|SetActiveStatus (Actor|GetComponentbyClass _array_element_3 "/Game/NPCManager/Blueprints/Characters/NPC/Comp_NPC_Controller.Comp_NPC_Controller_C") true)
            (Variables|/Game/NPCManager/Blueprints/Characters/NPC/Comp_NPC_Controller.Comp_NPC_Controller_C|SetPartialStatus (Actor|GetComponentbyClass _array_element_3 "/Game/NPCManager/Blueprints/Characters/NPC/Comp_NPC_Controller.Comp_NPC_Controller_C") false)
            (Variables|/Game/NPCManager/Blueprints/Characters/NPC/Comp_NPC_Controller.Comp_NPC_Controller_C|SetPrevPartialStatus (Actor|GetComponentbyClass _array_element_3 "/Game/NPCManager/Blueprints/Characters/NPC/Comp_NPC_Controller.Comp_NPC_Controller_C") false)
            (Default|EventSetInactiveOptions (Actor|GetComponentbyClass _array_element_3 "/Game/NPCManager/Blueprints/Characters/NPC/Comp_NPC_Controller.Comp_NPC_Controller_C") true)))))
    (:then_1
      ;[1 1 1] Partial Activate the NPCs
      (for _array_element_4 (Variables|Setup|GetPartialActiveNPCs)
        (Utilities|IsValid _array_element_4
          (:Is%20Valid
            (Variables|/Game/NPCManager/Blueprints/Characters/NPC/Comp_NPC_Controller.Comp_NPC_Controller_C|SetActiveStatus (Actor|GetComponentbyClass _array_element_4 "/Game/NPCManager/Blueprints/Characters/NPC/Comp_NPC_Controller.Comp_NPC_Controller_C") false)
            (Variables|/Game/NPCManager/Blueprints/Characters/NPC/Comp_NPC_Controller.Comp_NPC_Controller_C|SetPrevStatus (Actor|GetComponentbyClass _array_element_4 "/Game/NPCManager/Blueprints/Characters/NPC/Comp_NPC_Controller.Comp_NPC_Controller_C") false)
            (Variables|/Game/NPCManager/Blueprints/Characters/NPC/Comp_NPC_Controller.Comp_NPC_Controller_C|SetPartialStatus (Actor|GetComponentbyClass _array_element_4 "/Game/NPCManager/Blueprints/Characters/NPC/Comp_NPC_Controller.Comp_NPC_Controller_C") true)
            (Default|EventSetInactiveOptions (Actor|GetComponentbyClass _array_element_4 "/Game/NPCManager/Blueprints/Characters/NPC/Comp_NPC_Controller.Comp_NPC_Controller_C") false)))))
    (:then_2
      ;[1 1 1] Deactivate the NPCs
      (for _array_element_5 (Variables|Setup|GetInactiveNPCs)
        (Utilities|IsValid _array_element_5
          (:Is%20Valid
            (Variables|/Game/NPCManager/Blueprints/Characters/NPC/Comp_NPC_Controller.Comp_NPC_Controller_C|SetActiveStatus (Actor|GetComponentbyClass _array_element_5 "/Game/NPCManager/Blueprints/Characters/NPC/Comp_NPC_Controller.Comp_NPC_Controller_C") false)
            (Variables|/Game/NPCManager/Blueprints/Characters/NPC/Comp_NPC_Controller.Comp_NPC_Controller_C|SetPartialStatus (Actor|GetComponentbyClass _array_element_5 "/Game/NPCManager/Blueprints/Characters/NPC/Comp_NPC_Controller.Comp_NPC_Controller_C") false)
            (Variables|/Game/NPCManager/Blueprints/Characters/NPC/Comp_NPC_Controller.Comp_NPC_Controller_C|SetPrevStatus (Actor|GetComponentbyClass _array_element_5 "/Game/NPCManager/Blueprints/Characters/NPC/Comp_NPC_Controller.Comp_NPC_Controller_C") true)
            (Variables|/Game/NPCManager/Blueprints/Characters/NPC/Comp_NPC_Controller.Comp_NPC_Controller_C|SetPrevPartialStatus (Actor|GetComponentbyClass _array_element_5 "/Game/NPCManager/Blueprints/Characters/NPC/Comp_NPC_Controller.Comp_NPC_Controller_C") false)
            (Default|EventSetInactiveOptions (Actor|GetComponentbyClass _array_element_5 "/Game/NPCManager/Blueprints/Characters/NPC/Comp_NPC_Controller.Comp_NPC_Controller_C") true)))))))

(fn FnShowRenderStas
  (for _array_element (Variables|Setup|GetNPCList)
    (bind _output_get (LocalVariables|SetNPC _array_element))
    (Utilities|IsValid _output_get
      (:Is%20Valid
        ;[1 1 1] Has the NPC been rendered?
        (if (Variables|/Game/NPCManager/Blueprints/Characters/NPC/Comp_NPC_Controller.Comp_NPC_Controller_C|GetisRendered (Actor|GetComponentbyClass _output_get "/Game/NPCManager/Blueprints/Characters/NPC/Comp_NPC_Controller.Comp_NPC_Controller_C"))
          ;[1 1 1] Add to Render List
          (Utilities|Array|Add (LocalVariables|GetRenderedList) (LocalVariables|GetNPC))
          (else
            ;[1 1 1] Add to No Render List
            (Utilities|Array|Add (LocalVariables|GetNoRenderList) (LocalVariables|GetNPC)))))))
  (Utilities|FlowControl|Sequence
    (:then_0
      (Development|PrintString (Utilities|String|Append "NPCs Not Rendered: " (Utilities|String|ToString(Integer) (Utilities|Array|Length (LocalVariables|GetNoRenderList)))) true true "(R=0.000000,G=0.660000,B=1.000000,A=1.000000)" (Variables|Default|GetCheckRenderFreq)))
    (:then_1
      (Development|PrintString (Utilities|String|Append "NPCs Rendered: " (Utilities|String|ToString(Integer) (Utilities|Array|Length (LocalVariables|GetRenderedList)))) true true "(R=0.000000,G=0.660000,B=1.000000,A=1.000000)" (Variables|Default|GetCheckRenderFreq)))
    (:then_2
      (Development|PrintString "=================" true true "(R=0.000000,G=0.660000,B=1.000000,A=1.000000)" (Variables|Default|GetCheckRenderFreq))
      (Development|PrintString "Render Optimization" true true "(R=0.000000,G=0.660000,B=1.000000,A=1.000000)" (Variables|Default|GetCheckRenderFreq)))))

(fn FnAddPlayer
  (params (Player%20Pawn :type Actor%20Object%20Reference))
  (Utilities|Array|Add (Variables|Setup-Proximity|GetPlayerList) Player%20Pawn))

(event Custom|EventCheckTime
  (params (Hour :type Float%20%28single-precision%29))
  (bind _output_get (Variables|TOD|SetCurrentHour Hour))
  (Variables|TOD|SetWholeHour (Math|Float|Truncate _output_get))
  ;[1 1 1] Check for Authority
  (Networking|SwitchHasAuthority
    (:Authority
      (Utilities|FlowControl|Sequence
        (:then_0
          ;[1 1 1] Is the Whole Hour bigger than the Previous Hour?
          (if (> (Variables|TOD|GetWholeHour) (Variables|TOD|GetPrevHour))
            (Variables|Default|SetResetHour true)
            (Variables|TOD|SetPrevHour (Variables|TOD|GetWholeHour))
            (Default|CallDispNewHour :!label _label)
            (elif (== (Variables|TOD|GetWholeHour) 0)
              (if (Variables|Default|GetResetHour)
                (Variables|Default|SetResetHour false)
                (Variables|TOD|SetPrevHour 0)
                (goto _label)))))
        (:then_1
          ;[1 1 1] Check if the current hour is between DayStart and DayEnd
          (if (and (>= (Variables|TOD|GetCurrentHour) (Variables|TOD|GetDayStart)) (<= (Variables|TOD|GetCurrentHour) (Variables|TOD|GetDayEnd)))
            (Utilities|FlowControl|Sequence
              (:then_0
                (Utilities|FlowControl|DoOnce false :!label _label_2
                  (:Completed
                    (Default|CallDispDayStarted))))
              (:then_1
                (goto _label_3 Reset)))
            (else
              (Utilities|FlowControl|Sequence
                (:then_0
                  (Utilities|FlowControl|DoOnce false :!label _label_3
                    (:Completed
                      (Default|CallDispDayEnded))))
                (:then_1
                  (goto _label_2 Reset))))))))))