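; BP_DialogueZone is a placeable zone that changes the dialogue options of NPCs inside it.
; When activated, it replaces, adds or removes its dialogue entries according to ExecutionMode, with separate events for calling each operation directly.
; Each operation box-traces the Trigger bounds for Pawns with a Comp_NPC_Controller and passes the entries to that component.
; The construction script applies trigger scale and visibility settings.
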(event Custom|Replace%20Dialogue
  (CallFunction|FnReplaceDialogue))

(event Custom|Add%20Dialogue
  (CallFunction|FnAddRemoveDialogue true))

(event Custom|Remove%20Dialogue
  (CallFunction|FnAddRemoveDialogue false))

(event Custom|EventActivate
  (switch Utilities|FlowControl|Switch|SwitchonEnum_DialogueZone_ExecMode (Variables|Setup|GetExecutionMode)
    (:NewEnumerator0
      (CallFunction|FnReplaceDialogue))
    (:NewEnumerator1
      (CallFunction|FnAddRemoveDialogue true))
    (:NewEnumerator2
      (CallFunction|FnAddRemoveDialogue false))))

(fn ConstructionScript
  ;[1 1 1] Set trigger scale and visibility
  (Transformation|SetWorldScale3D (Variables|Default|GetTrigger) (Variables|Setup|GetTriggerScale))
  (Rendering|SetVisibility (Variables|Default|GetTrigger) (Variables|Setup|GetTriggerVisibility) false)
  (Development|SetHiddeninGame (Variables|Default|GetTrigger) (Variables|Setup|GetTriggerHidden) false))

(fn FnTraceforNPCs
  (bind _trigger (Variables|Default|GetTrigger))
  (bind _returnvalue (Transformation|GetWorldLocation _trigger))
  ;[1 1 1] Trace for NPCs
  (bind (_outhits _returnvalue_2) (Class|KismetSystemLibrary|BoxTraceMultiforObjects _returnvalue (+ _returnvalue "0, 0,0.010000") (.BoxExtent (Collision|GetComponentBounds _trigger)) (Transformation|GetWorldRotation _trigger) (Utilities|Array|MakeArray "ObjectTypeQuery3") false 0 (select (Variables|Setup|GetDebugTrace) "ForDuration" "None") true))
  (if _returnvalue_2
    (for _array_element _outhits
      ;[1 1 1] Does the Hit Actor contain the NPC Controller component?
      (bind _output_get (LocalVariables|SetHitActor (.HitActor (Collision|BreakHitResult _array_element))))
      (Utilities|IsValid (Actor|GetComponentbyClass _output_get "/Game/NPCManager/Blueprints/Characters/NPC/Comp_NPC_Controller.Comp_NPC_Controller_C")
        (:Is%20Valid
          ;[1 1 1] Add NPC to the list
          (Utilities|Array|Add (LocalVariables|GetNPCList) (LocalVariables|GetHitActor)))))
    (return (LocalVariables|GetNPCList))))

(fn FnReplaceDialogue
  ;[1 1 1] Loop through all the NPCs
  (for _array_element (CallFunction|FnTraceforNPCs)
    (bind _output_get (LocalVariables|SetNPC _array_element))
    (Utilities|IsValid _output_get
      (:Is%20Valid
        ;[1 1 1] Set the Dialogue Entries as the new Dialogue options for this NPC
        (Class|BPINPCInteraction|FnSetAllowedDialogue(Message) (Actor|GetComponentbyClass (LocalVariables|GetNPC) "/Game/NPCManager/Blueprints/Characters/NPC/Comp_NPC_Controller.Comp_NPC_Controller_C") (Variables|Setup|GetGreetingsGoodbyes) (Variables|Setup|GetDialogueEntries))))))

(fn FnAddRemoveDialogue
  (params (Add :type Boolean))
  (LocalVariables|SetA Add)
  ;[1 1 1] Loop through all the NPCs
  (for _array_element (CallFunction|FnTraceforNPCs)
    (LocalVariables|SetNPC _array_element)
    ;[1 1 1] Add or remove dialogue options for this NPC
    (Class|BPINPCInteraction|FnAddRemoveDialogue(Message) (Actor|GetComponentbyClass (LocalVariables|GetNPC) "/Game/NPCManager/Blueprints/Characters/NPC/Comp_NPC_Controller.Comp_NPC_Controller_C") (LocalVariables|GetA) (Variables|Setup|GetGreetingsGoodbyes) (Variables|Setup|GetDialogueEntries))))