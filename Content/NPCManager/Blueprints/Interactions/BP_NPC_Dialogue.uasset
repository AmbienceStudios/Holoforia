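; Proximity-triggered NPC dialogue actor that displays lines on a screen widget and plays their audio with attenuation.
; It creates the dialogue widget on BeginPlay, then shows or hides it as the local player enters or leaves a configurable sphere trigger.
; The NPC Manager's ShowingDialogue flag, updated on show and hide, blocks showing while another dialogue is active.
; Functions set name and text, play or stop clips, and optionally log lines to a lazily created debug widget.
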(event OnComponentBeginOverlap(Trigger)
  (params (OverlappedComponent :type Primitive%20Component%20Object%20Reference) (OtherActor :type Actor%20Object%20Reference) (OtherComp :type Primitive%20Component%20Object%20Reference) (OtherBodyIndex :type Integer) (bFromSweep :type Boolean) (SweepResult :type Hit%20Result%20Structure%20%28by%20ref%29))
  (bind _instigator (Variables|/Script/Engine.Actor|GetInstigator OtherActor))
  (bind _returnvalue (Pawn|GetController _instigator))
  ;[1 1 1] Are we overlapping the Player?
  (Utilities|IsValid _returnvalue
    (:Is%20Valid
      (if (Pawn|IsLocalPlayerController _returnvalue)
        (Utilities|IsValid (Variables|Setup|GetNPCManager)
          (:Is%20Valid
            (if (not (Variables|/Game/NPCManager/Blueprints/BP_NPC_Manager.BP_NPC_Manager_C|GetShowingDialogue (Variables|Setup|GetNPCManager)))
              ;[1 1 1] Show the widget
              (CallFunction|EventShowHideWidget true :!label _label)))
          (:Is%20Not%20Valid
            (goto _label)))))))

(event OnComponentEndOverlap(Trigger)
  (params (OverlappedComponent :type Primitive%20Component%20Object%20Reference) (OtherActor :type Actor%20Object%20Reference) (OtherComp :type Primitive%20Component%20Object%20Reference) (OtherBodyIndex :type Integer))
  (bind _instigator (Variables|/Script/Engine.Actor|GetInstigator OtherActor))
  (bind _returnvalue (Pawn|GetController _instigator))
  ;[1 1 1] Are we overlapping the Player?
  (Utilities|IsValid _returnvalue
    (:Is%20Valid
      (if (Pawn|IsLocalPlayerController _returnvalue)
        ;[1 1 1] Hide the widget
        (CallFunction|EventShowHideWidget false)))))

(event Custom|EventCreateWidget
  (CallFunction|FnCreateWidget))

(event Custom|EventShowHideWidget
  (params (Show :type Boolean))
  (CallFunction|FnShowHideWidget Show))

(event EventBeginPlay
  (CallFunction|EventCreateWidget)
  ;[1 1 1] Set audio attenuation settings
  (Variables|/Script/Engine.AudioComponent|SetAttenuationSettings (Variables|Default|GetAudio) "/Game/NPCManager/Sound/Dialogue/SA_NPC_Dialogue.SA_NPC_Dialogue"))

(fn ConstructionScript
  ;[1 1 1] Set the Trigger radius
  (Components|Sphere|SetSphereRadius (Variables|Default|GetTrigger) (Variables|Setup|GetTriggerRadius) true))

(fn FnCreateWidget
  ;[1 1 1] Spawn the NPC Dialogue widget and add it to the screen
  (bind _returnvalue (UserInterface|CreateWidget "/Game/NPCManager/Blueprints/Widgets/WBP_NPC_Dialogue.WBP_NPC_Dialogue_C" (Game|GetPlayerController 0)))
  (bind _output_get (Variables|Setup|SetWidgetRef _returnvalue))
  (Utilities|IsValid _output_get
    (:Is%20Valid
      (UserInterface|Viewport|AddtoPlayerScreen _output_get))))

(fn FnShowHideWidget
  (params (Show :type Boolean))
  (bind _npcmanager (Variables|Setup|GetNPCManager))
  (LocalVariables|SetS Show)
  (Utilities|IsValid (Variables|Setup|GetWidgetRef)
    (:Is%20Valid
      ;[1 1 1] Show or Hide the dialogue widget
      (Default|FnShowHideWidget (Variables|Setup|GetWidgetRef) (LocalVariables|GetS))
      ;[1 1 1] Set ShowingDialogue value in the NPC Manager
      (Utilities|IsValid _npcmanager
        (:Is%20Valid
          (Variables|/Game/NPCManager/Blueprints/BP_NPC_Manager.BP_NPC_Manager_C|SetShowingDialogue _npcmanager (LocalVariables|GetS)))))))

(fn FnPlaySound
  (params (Audio%20Clip :type Sound%20Base%20Object%20Reference))
  (LocalVariables|SetSound Audio%20Clip)
  ;[1 1 1] Stop playing
  (Audio|Components|Audio|Stop (Variables|Default|GetAudio))
  ;[1 1 1] Set the new sound and play it
  (Audio|Components|Audio|SetSound (Variables|Default|GetAudio) (LocalVariables|GetSound))
  (Audio|Components|Audio|Play (Variables|Default|GetAudio) 0.0))

(fn FnStopSound
  ;[1 1 1] Stop playing
  (Audio|Components|Audio|Stop (Variables|Default|GetAudio)))

(fn FnDisplayLine
  (params (NPC%20Name :type Text) (New%20Line :type Struct%20DT%20NPC%20Dialogue%20Structure) (Debug%20Line :type Boolean) (Line%20State :type Enum_NPC_Dialogue_State%20Enum :default "NewEnumerator0"))
  (LocalVariables|SetName NPC%20Name)
  (LocalVariables|SetLine New%20Line)
  (LocalVariables|SetDebug Debug%20Line)
  (LocalVariables|SetState Line%20State)
  (Utilities|FlowControl|Sequence
    (:then_0
      (Utilities|IsValid (Variables|Setup|GetWidgetRef)
        (:Is%20Valid
          ;[1 1 1] Set the Name and Dialogue line on the widget
          (Default|FnSetName (Variables|Setup|GetWidgetRef) (LocalVariables|GetName))
          (Default|FnSetDialogue (Variables|Setup|GetWidgetRef) (Utilities|Struct|BreakStruct_DT_NPC_Dialogue (LocalVariables|GetLine))))))
    (:then_1
      (if (LocalVariables|GetDebug)
        ;[1 1 1] Do we already have a debug widget?
        (Utilities|IsValid (Variables|Default|GetWidgetDebugDialog)
          (:Is%20Valid
            _)
          (:Is%20Not%20Valid
            ;[1 1 1] Create debug widget and add to viewport
            (bind _returnvalue (UserInterface|CreateWidget "/Game/NPCManager/Blueprints/Widgets/WBP_NPC_DebugDialogue.WBP_NPC_DebugDialogue_C" (Game|GetPlayerController 0)))
            (bind _output_get (Variables|Default|SetWidgetDebugDialog _returnvalue))
            (Utilities|IsValid _output_get
              (:Is%20Valid
                (UserInterface|Viewport|AddtoPlayerScreen _output_get)))))
        ;[1 1 1] Add the line to the widget
        (Default|FnAddLine (Variables|Default|GetWidgetDebugDialog) (LocalVariables|GetName) (LocalVariables|GetLine) (LocalVariables|GetState))))))