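; Diagnostic actor that checks a level's NPC Manager setup and prints a troubleshooting report.
; One second after BeginPlay, or via RunTroubleshooter, it checks for nav mesh bounds, the manager, player tag and component, and NPC-tagged actors lacking controllers.
; The report also flags bounding boxes, waypoints and paths whose collision object type isn't NPC_Navigation.
; Lines print in reverse, footer first and title last, suiting newest-on-top screen messages.
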(event Custom|Run%20Troubleshooter
  (CallFunction|FnCheckLevel))

(event EventBeginPlay
  (Utilities|FlowControl|Delay 1.0)
  (CallFunction|FnCheckLevel))

(fn ConstructionScript)

(fn FnCheckLevel
  (Utilities|FlowControl|Sequence
    (:then_0
      ;[1 1 1] Check for a Nav Mesh in the level
      (bind _outactors (Actor|GetAllActorsOfClass "/Script/NavigationSystem.NavMeshBoundsVolume"))
      (if (Utilities|Array|IsValidIndex _outactors)
        (LocalVariables|SetFoundNavMesh true)
        (else
          (LocalVariables|SetFoundNavMesh false))))
    (:then_1
      ;[1 1 1] Check for the NPC Manager BP in the level
      (bind _outactors_2 (Actor|GetAllActorsOfClass "/Game/NPCManager/Blueprints/BP_NPC_Manager.BP_NPC_Manager_C"))
      (if (Utilities|Array|IsValidIndex _outactors_2)
        (LocalVariables|SetFoundManager true)
        (else
          (LocalVariables|SetFoundManager false))))
    (:then_2
      ;[1 1 1] Check for Player Tag
      (if (Utilities|Array|ContainsItem (Variables|/Script/Engine.Actor|GetTags (Game|Player|GetPlayerPawn 0)) "Player")
        (LocalVariables|SetPlayerTagFound true)
        (else
          (LocalVariables|SetPlayerTagFound false))))
    (:then_3
      ;[1 1 1] Check that the Player has the Player NPC Check component
      (Utilities|IsValid (Actor|GetComponentbyClass (Game|Player|GetPlayerPawn 0) "/Game/NPCManager/Blueprints/Characters/Player/Comp_Player_NPCCheck.Comp_Player_NPCCheck_C")
        (:Is%20Valid
          (LocalVariables|SetFoundPlayerComp true))
        (:Is%20Not%20Valid
          (LocalVariables|SetFoundPlayerComp false))))
    (:then_4
      ;[1 1 1] Loop through all the NPCs in the scene
      (bind _outactors_3 (Actor|GetAllActorswithTag "NPC"))
      (bind _output_get (LocalVariables|SetNPCs _outactors_3))
      (for _array_element _output_get
        (bind _output_get_2 (LocalVariables|SetNPC _array_element))
        ;[1 1 1] Check that this NPC does NOT have the controller component and is NOT the Player
        (if (and (not (Utilities|IsValid (Actor|GetComponentbyClass _output_get_2 "/Game/NPCManager/Blueprints/Characters/NPC/Comp_NPC_Controller.Comp_NPC_Controller_C"))) (!= (Game|Player|GetPlayerPawn 0) (LocalVariables|GetNPC)))
          ;[1 1 1] Add this NPC to the list
          (Utilities|Array|Add (LocalVariables|GetBadNPCs) (LocalVariables|GetNPC)))))
    (:then_5
      (|PRINTREPORT))))

(fn FnCheckBoundingBoxes
  (bind _outactors (Actor|GetAllActorsOfClass "/Game/NPCManager/Blueprints/Navigaton/BP_NPC_BoundingBox.BP_NPC_BoundingBox_C"))
  (for _array_element _outactors
    (bind _output_get (LocalVariables|SetBounds _array_element))
    (if (not (Utilities|Enum|Equal(Enum) (Utilities|String|EnumtoString (Collision|GetCollisionObjectType (Variables|/Game/NPCManager/Blueprints/Navigaton/BP_NPC_BoundingBox.BP_NPC_BoundingBox_C|GetBounds _output_get))) "NPC_Navigation"))
      (Development|PrintString (Utilities|String|Append (Utilities|GetDisplayName (LocalVariables|GetBounds)) (LocalVariables|GetErrorMessage)) true true "(R=1.000000,G=0.000000,B=0.000000,A=1.000000)" (Variables|Default|GetReportDuration))
      (LocalVariables|SetError true)))
  (if (not (LocalVariables|GetError))
    (Development|PrintString "NPC Bounding Boxes: No Errors Detected" true true "(R=0.000000,G=0.660000,B=0.000000,A=1.000000)" (Variables|Default|GetReportDuration))))

(fn FnCheckWayPoints
  (bind _outactors (Actor|GetAllActorsOfClass "/Game/NPCManager/Blueprints/Navigaton/BP_NPC_WayPoint.BP_NPC_WayPoint_C"))
  (for _array_element _outactors
    (bind _output_get (LocalVariables|SetWayPoint _array_element))
    (if (not (Utilities|Enum|Equal(Enum) (Utilities|String|EnumtoString (Collision|GetCollisionObjectType (Variables|/Game/NPCManager/Blueprints/Navigaton/BP_NPC_WayPoint.BP_NPC_WayPoint_C|GetSphere _output_get))) "NPC_Navigation"))
      (Development|PrintString (Utilities|String|Append (Utilities|GetDisplayName (LocalVariables|GetWayPoint)) (LocalVariables|GetErrorMessage)) true true "(R=1.000000,G=0.000000,B=0.000000,A=1.000000)" (Variables|Default|GetReportDuration))
      (LocalVariables|SetError true)))
  (if (not (LocalVariables|GetError))
    (Development|PrintString "NPC Way Points: No Errors Detected" true true "(R=0.000000,G=0.660000,B=0.000000,A=1.000000)" (Variables|Default|GetReportDuration))))

(fn FnCheckPaths
  (bind _outactors (Actor|GetAllActorsOfClass "/Game/NPCManager/Blueprints/Navigaton/BP_NPC_Path.BP_NPC_Path_C"))
  (for _array_element _outactors
    (bind _output_get (LocalVariables|SetPath _array_element))
    (if (not (Utilities|Enum|Equal(Enum) (Utilities|String|EnumtoString (Collision|GetCollisionObjectType (Variables|/Game/NPCManager/Blueprints/Navigaton/BP_NPC_Path.BP_NPC_Path_C|GetSphere _output_get))) "NPC_Navigation"))
      (Development|PrintString (Utilities|String|Append (Utilities|GetDisplayName (LocalVariables|GetPath)) (LocalVariables|GetErrorMessage)) true true "(R=1.000000,G=0.000000,B=0.000000,A=1.000000)" (Variables|Default|GetReportDuration))
      (LocalVariables|SetError true)))
  (if (not (LocalVariables|GetError))
    (Development|PrintString "NPC Paths: No Errors Detected" true true "(R=0.000000,G=0.660000,B=0.000000,A=1.000000)" (Variables|Default|GetReportDuration))))