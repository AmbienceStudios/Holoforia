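; BP_CameraActor is a utility camera that, when Active, becomes the player's view and tours an array of target actors.
; Mouse axes orbit the CameraBoom with clamped pitch (InvertYaw actually flips pitch), and the wheel changes arm length to zoom.
; E glides to the current target through a timeline using that target's MovementRate, while Q teleports there.
; Both then advance the index, wrapping to the first.
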(event EventBeginPlay
  (if (Variables|Setup|GetActive)
    ;[1 1 1] Invert Yaw controls?
    (if (Variables|Setup|GetInvertYaw?)
      (Variables|Default|SetYawDirection -1.0)
      (else
        (Variables|Default|SetYawDirection 1.0)))
    (Game|Player|SetViewTargetwithBlend (Game|GetPlayerController 0) self 1.0 "VTBlend_Linear" 0.0 false)
    (else
      ;[1 1 1] BP not active, do not consume input
      (Input|DisableInput self (Game|GetPlayerController 0)))))

(event Input|AxisEvents|InputAxisLookUp
  (params (AxisValue :type Float%20%28single-precision%29))
  (bind _cameraboom (Variables|Default|GetCameraBoom))
  (bind _relativerotation (Variables|/Script/Engine.SceneComponent|GetRelativeRotation _cameraboom))
  ;[1 1 1] Rotate camera by moving the Mouse
  (Transformation|SetRelativeRotation (Variables|Default|GetCameraBoom) (Math|Rotator|MakeRotator (.roll _relativerotation) (Math|Float|Clamp(Float) (+ (.pitch _relativerotation) (* AxisValue 2.0 (Variables|Default|GetYawDirection))) -89.0 89.0) (.yaw _relativerotation)) false false))

(event Input|AxisEvents|InputAxisTurn
  (params (AxisValue :type Float%20%28single-precision%29))
  (bind _cameraboom (Variables|Default|GetCameraBoom))
  (bind _relativerotation (Variables|/Script/Engine.SceneComponent|GetRelativeRotation _cameraboom))
  ;[1 1 1] Rotate camera by moving the Mouse
  (Transformation|SetRelativeRotation (Variables|Default|GetCameraBoom) (Math|Rotator|MakeRotator (.roll _relativerotation) (.pitch _relativerotation) (+ (.yaw _relativerotation) (* AxisValue 2.0))) false false))

(event Input|MouseEvents|MouseWheelUp
  (params (Key :type Key%20Structure))
  ;[1 1 1] Zoom In and Out
  (:Pressed
    (Variables|/Script/Engine.SpringArmComponent|SetTargetArmLength (Variables|Default|GetCameraBoom) (- (Variables|/Script/Engine.SpringArmComponent|GetTargetArmLength (Variables|Default|GetCameraBoom)) (Variables|Default|GetZoomAmount)))))

(event Input|MouseEvents|MouseWheelDown
  (params (Key :type Key%20Structure))
  ;[1 1 1] Zoom In and Out
  (:Pressed
    (Variables|/Script/Engine.SpringArmComponent|SetTargetArmLength (Variables|Default|GetCameraBoom) (+ (Variables|/Script/Engine.SpringArmComponent|GetTargetArmLength (Variables|Default|GetCameraBoom)) (Variables|Default|GetZoomAmount)))))

(event Input|KeyboardEvents|E
  (params (Key :type Key%20Structure))
  (bind _targets (Variables|Setup|GetTargets))
  (bind _currenttarget (Variables|Default|GetCurrentTarget))
  (bind _output (Utilities|Array|Get(acopy) _targets _currenttarget))
  (bind _returnvalue (Transformation|GetActorTransform _output))
  ;[1 1 1] GO TO TARGET
  (:Pressed
    (Variables|Default|SetStart (Transformation|GetActorTransform))
    (Components|Timeline|SetPlayRate (Variables|Default|GetTM_Movement) (Variables|/Game/NPCManager/Blueprints/Utilities/Camera/BP_CameraTarget.BP_CameraTarget_C|GetMovementRate (Utilities|Array|Get(acopy) (Variables|Setup|GetTargets) (Variables|Default|GetCurrentTarget))))
    (bind _alpha (Timeline|TM_Movement PlayFromStart)
      (:Update
        (Transformation|SetActorLocationAndRotation (Math|Vector|Lerp(Vector) (.location (Variables|Default|GetStart)) (.location _returnvalue) _alpha) (Math|Rotator|Lerp(Rotator) (.rotation (Variables|Default|GetStart)) (.rotation _returnvalue) _alpha) false true))
      (:Finished
        (|NEXTTARGET_2)))))

(event Input|KeyboardEvents|Q
  (params (Key :type Key%20Structure))
  (bind _start (Variables|Default|GetStart))
  (bind _targets (Variables|Setup|GetTargets))
  (bind _currenttarget (Variables|Default|GetCurrentTarget))
  (bind _targets_2 (Variables|Setup|GetTargets))
  (bind _currenttarget_2 (Variables|Default|GetCurrentTarget))
  (bind _output (Utilities|Array|Get(acopy) _targets _currenttarget))
  (bind _output_2 (Utilities|Array|Get(acopy) _targets_2 _currenttarget_2))
  (bind _returnvalue (Transformation|GetActorTransform _output))
  (bind _returnvalue_2 (Transformation|GetActorTransform _output_2))
  ;[1 1 1] TELEPORT TO TARGET
  (:Pressed
    (Utilities|FlowControl|Sequence
      (:then_0
        (bind _alpha (Timeline|TM_Movement Stop)
          (:Update
            (Transformation|SetActorLocationAndRotation (Math|Vector|Lerp(Vector) (.location _start) (.location _returnvalue) _alpha) (Math|Rotator|Lerp(Rotator) (.rotation _start) (.rotation _returnvalue) _alpha) false true))
          (:Finished
            (|NEXTTARGET_2))))
      (:then_1
        (Transformation|SetActorLocationAndRotation (.location _returnvalue_2) (.rotation _returnvalue_2) false true)
        (|NEXTTARGET)))))

(fn ConstructionScript)