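; Day/night cycle actor that runs a 24-hour game clock, scaled from a configurable day length, to drive the sun and NPC schedules.
; The authority advances the hour each Tick, passes it to the NPC Manager and, unless DataOnly, updates SunAngle.
; SunAngle's RepNotify rotates the sun, updates the skydome and recaptures the skylight.
; Time can be paused, resumed, queried or shown in a debug widget.
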(event Custom|Pause%20Time
  ;[1 1 1] Blutilities to Pause and Resume time calculations
  (Variables|Default|SetCalculateTime false))

(event Custom|Resume%20Time
  ;[1 1 1] Blutilities to Pause and Resume time calculations
  (Variables|Default|SetCalculateTime true))

(event EventBeginPlay
  ;[1 1 1] Check for Authority
  (Networking|SwitchHasAuthority
    (:Authority
      (|CALCULATETIMEVARIABLES)
      (|NPCMANAGER
        (:Is%20Valid
          (if (Variables|Setup|GetDebugTime)
            ;[1 1 1] Create Time widget and add it to the viewport
            (bind _returnvalue (UserInterface|CreateWidget "/Game/NPCManager/Blueprints/Widgets/WBP_DebugTime.WBP_DebugTime_C"))
            (bind _output_get (Variables|Default|SetTimeWidget _returnvalue))
            (Utilities|IsValid _output_get
              (:Is%20Valid
                (UserInterface|Viewport|AddtoViewport _output_get 0)))))))))

(event EventTick
  (params (DeltaSeconds :type Float%20%28single-precision%29))
  (Variables|Default|SetDeltaTime DeltaSeconds)
  (Utilities|FlowControl|Sequence
    (:then_0
      ;[1 1 1] Check for Authority
      (Networking|SwitchHasAuthority
        (:Authority
          ;[1 1 1] Are we Active and calculating time?
          (if (and (Variables|Setup|GetActive?) (Variables|Default|GetCalculateTime))
            (Utilities|IsValid (Variables|Setup|GetNPCManager)
              (:Is%20Valid
                (Default|EventCheckTime (Variables|Setup|GetNPCManager) (Variables|Time|GetCurrentHour)))
              (:Is%20Not%20Valid
                _))
            ;[1 1 1] Calculate current Hour of the Day
            (Variables|Time|SetCurrentHour (+ (Variables|Time|GetCurrentHour) (/ (Variables|Default|GetDeltaTime) (Variables|Time|GetOneHour))))
            ;[1 1 1] Is this NOT a Data Only BP?
            (if (not (Variables|Setup|GetDataOnly))
              ;[1 1 1] Calculate Sun Angle
              (Variables|SunPosition|SetSunAngle (+ (* (/ (Variables|Time|GetCurrentHour) 6.0) 9e+01) 9e+01)))
            ;[1 1 1] Reset Hour to 0 after 24 hours
            (if (> (Variables|Time|GetCurrentHour) 24.0)
              (Variables|Time|SetCurrentHour 0.0))))))
    (:then_1
      ;[1 1 0] DEBUG
      (if (Variables|Setup|GetDebugTime)
        (Utilities|IsValid (Variables|Default|GetTimeWidget)
          (:Is%20Valid
            (Default|FnSetTime (Variables|Default|GetTimeWidget) (Variables|Time|GetCurrentHour))))))))

(fn ConstructionScript)

(fn OnRepSunAngle
  (Utilities|IsValid (Variables|SunPosition|GetSunRef)
    (:Is%20Valid
      ;[1 1 1] Rotate the sun
      (Transformation|SetActorRotation (Variables|SunPosition|GetSunRef) (Math|Rotator|MakeRotator 0.0 (Variables|SunPosition|GetSunAngle) 0.0)))
    (:Is%20Not%20Valid
      ;[1 1 1] No Sun reference found!
      (Development|PrintString "No Sun Reference Found" true true "(R=1.000000,G=0.000000,B=0.000000,A=1.000000)" 5.0)))
  (Utilities|IsValid (Variables|SunPosition|GetSkyDomeRef)
    (:Is%20Valid
      ;[1 1 1] Update Skydome
      (Default|UpdateSunDirection (Variables|SunPosition|GetSkyDomeRef)))
    (:Is%20Not%20Valid
      ;[1 1 1] No Skydome reference found!
      (Development|PrintString "No Skydome Reference Found" true true "(R=1.000000,G=0.000000,B=0.000000,A=1.000000)" 5.0)))
  (Utilities|IsValid (Variables|SunPosition|GetSkylightRef)
    (:Is%20Valid
      ;[1 1 1] Recapture the sky
      (Class|SkyLightComponent|RecaptureSky (Variables|/Script/Engine.SkyLight|GetLightComponent (Variables|SunPosition|GetSkylightRef))))))

(fn FnGetHourDuration
  (return (Variables|Time|GetOneHour)))

(fn FnGetTime
  (return (Variables|Time|GetCurrentHour)))