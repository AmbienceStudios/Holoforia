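; Showcase trigger actor that opens a door and changes an NPC's task when the Player-tagged actor enters it.
; A DoOnce gates the overlap and re-arms when the player leaves.
; A timeline lerps the door from its current location to a final location.
; The NPC's Comp_NPC_Controller_CustomLogic component gets a new assigned task and is told to start it through EventNextTask.
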(event OnComponentBeginOverlap(Trigger)
  (params (OverlappedComponent :type Primitive%20Component%20Object%20Reference) (OtherActor :type Actor%20Object%20Reference) (OtherComp :type Primitive%20Component%20Object%20Reference) (OtherBodyIndex :type Integer) (bFromSweep :type Boolean) (SweepResult :type Hit%20Result%20Structure%20%28by%20ref%29))
  (bind _npc (Variables|Setup|GetNPC))
  (bind _returnvalue (Actor|GetComponentbyClass _npc "/Game/NPCManager/Blueprints/Characters/NPC/CustomLogic/Comp_NPC_Controller_CustomLogic.Comp_NPC_Controller_CustomLogic_C"))
  ;[1 1 1] Check that the Player is overlapping
  (if (Actor|ActorHasTag OtherActor "Player")
    (Utilities|IsValid (Variables|Setup|GetNPC)
      (:Is%20Valid
        ;[1 1 1] Check that the NPC has the correct component
        (Utilities|IsValid _returnvalue
          (:Is%20Valid
            (Variables|Default|SetNPCController _returnvalue))))
      (:Is%20Not%20Valid
        _))
    (Utilities|FlowControl|DoOnce false
      (:Completed
        (Utilities|FlowControl|Sequence
          (:then_0
            (CallFunction|EventOpenDoor))
          (:then_1
            (CallFunction|EventChangeTask)))))))

(event OnComponentEndOverlap(Trigger)
  (params (OverlappedComponent :type Primitive%20Component%20Object%20Reference) (OtherActor :type Actor%20Object%20Reference) (OtherComp :type Primitive%20Component%20Object%20Reference) (OtherBodyIndex :type Integer))
  ;[1 1 1] Check that the Player is overlapping
  (if (Actor|ActorHasTag OtherActor "Player")
    (Utilities|FlowControl|DoOnce false) ; enters at Reset
  ))

(event Custom|EventOpenDoor
  (Variables|Default|SetDoorLocation (Transformation|GetActorLocation (Variables|Setup|GetDoor)))
  (bind _alpha (Timeline|TM_OpenDoor PlayFromStart)
    (:Update
      (Transformation|SetActorLocation (Variables|Setup|GetDoor) (Math|Vector|Lerp(Vector) (Variables|Default|GetDoorLocation) (Variables|Setup|GetFinalDoorLocation) _alpha) false true))))

(event Custom|EventChangeTask
  (Utilities|IsValid (Variables|Default|GetNPCController)
    (:Is%20Valid
      (Variables|/Game/NPCManager/Blueprints/Characters/NPC/CustomLogic/Comp_NPC_Controller_CustomLogic.Comp_NPC_Controller_CustomLogic_C|SetAssignedTask (Variables|Default|GetNPCController) 1)
      (Default|EventNextTask (Variables|Default|GetNPCController)))))

(fn ConstructionScript)