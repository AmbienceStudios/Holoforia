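; Showcase trigger actor that stages a one-shot explosion when an actor tagged Player enters its trigger.
; It spawns explosion emitters and sound at listed scene actors, enables physics on listed meshes, and fires radial force impulses.
; It also activates a dialogue zone to change NPC dialogue categories.
; Two delays, both starting at the blast, time the secondary smoke emitters and the cleanup of all spawned particles.
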(event OnComponentBeginOverlap(Trigger)
  (params (OverlappedComponent :type Primitive%20Component%20Object%20Reference) (OtherActor :type Actor%20Object%20Reference) (OtherComp :type Primitive%20Component%20Object%20Reference) (OtherBodyIndex :type Integer) (bFromSweep :type Boolean) (SweepResult :type Hit%20Result%20Structure%20%28by%20ref%29))
  ;[1 1 1] Check that the Player overlapped
  (if (Actor|ActorHasTag OtherActor "Player")
    ;[1 1 1] Spawn explosions
    (Utilities|FlowControl|DoOnce false
      (:Completed
        (CallFunction|EventCreateExplosions)))))

(fn ConstructionScript)

(event Custom|EventCreateExplosions
  (Utilities|FlowControl|Sequence
    (:then_0
      ;[1 1 1] Spawn particles
      (for _array_element (Variables|Setup|GetSceneActorList)
        (bind _output_get (Variables|Default|SetActor _array_element))
        (bind _returnvalue (Effects|SpawnEmitteratLocation (Variables|Setup|GetFirstEmitter) (.location (Transformation|GetActorTransform _output_get)) (.rotation (Transformation|GetActorTransform _output_get)) "5.000000,5.000000,5.000000"))
        (Utilities|Array|Add (Variables|Default|GetSpawnedParticles) _returnvalue)
        ;[1 1 1] Play explosion sound effect
        (Audio|PlaySoundatLocation (Variables|Setup|GetExplosionSound) (Transformation|GetActorLocation (Variables|Default|GetActor)) "0, 0, 0" 0.2 1.0 0.0 0 0 0)))
    (:then_1
      ;[1 1 1] Simulate physics
      (for _array_element_2 (Variables|Setup|GetSimulatePhysicsList)
        (Physics|SetSimulatePhysics (Actor|GetComponentbyClass _array_element_2 "/Script/Engine.StaticMeshComponent") true)))
    (:then_2
      ;[1 1 1] Spawn radial impulses
      (for _array_element_3 (Variables|Setup|GetRadialForceList)
        (Utilities|IsValid (Actor|GetComponentbyClass _array_element_3 "/Script/Engine.RadialForceComponent")
          (:Is%20Valid
            (Class|RadialForceComponent|FireImpulse (Actor|GetComponentbyClass _array_element_3 "/Script/Engine.RadialForceComponent"))))))
    (:then_3
      ;[1 1 1] Activate the Dialogue Zone to change the NPC dialogue categories
      (Utilities|IsValid (Variables|Setup|GetDialogueZone)
        (:Is%20Valid
          (Variables|/Game/NPCManager/Blueprints/Interactions/BP_DialogueZone.BP_DialogueZone_C|SetExecutionMode (Variables|Setup|GetDialogueZone) (Variables|Setup|GetDialogueExecutionMode))
          (Default|EventActivate (Variables|Setup|GetDialogueZone)))))
    (:then_4
      ;[1 1 1] Spawn the smoke
      (Utilities|FlowControl|Delay (Variables|Setup|GetSecondaryDelay))
      (for _array_element_4 (Variables|Setup|GetSceneActorList)
        (bind _output_get_2 (Variables|Default|SetActor _array_element_4))
        (bind _returnvalue_2 (Effects|SpawnEmitteratLocation (Variables|Setup|GetSecondEmitter) (.location (Transformation|GetActorTransform _output_get_2)) (.rotation (Transformation|GetActorTransform _output_get_2)) "5.000000,5.000000,5.000000"))
        (Utilities|Array|Add (Variables|Default|GetSpawnedParticles) _returnvalue_2)))
    (:then_5
      ;[1 1 1] Destroy the smoke particles
      (Utilities|FlowControl|Delay (Variables|Setup|GetDespawnDelay))
      (for _array_element_5 (Variables|Default|GetSpawnedParticles)
        (Utilities|IsValid _array_element_5
          (:Is%20Valid
            (Components|DestroyComponent _array_element_5)))))))