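; BP_LivingRoom is a showcase living room actor with couches, a table and floor lamps that changes appearance when interacted with.
; FnInteract runs through a DoOnce into EventActivate, so the change fires only once through that path.
; EventActivate swaps the furniture to changed materials and raises the intensity of two point lights to light the room.
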(event Custom|EventActivate
  ;[1 1 1] Change materials
  (Rendering|Material|SetMaterial (Variables|Default|GetCouch1) 0 "/Game/NPCManager/EpicContent/Materials/Livingroom/MI_Couch_NOSSS_Mat_Changed.MI_Couch_NOSSS_Mat_Changed")
  (Rendering|Material|SetMaterial (Variables|Default|GetTable) 0 "/Game/NPCManager/EpicContent/Materials/Livingroom/M_CoffeTable_MAT_Changed.M_CoffeTable_MAT_Changed")
  (Rendering|Material|SetMaterial (Variables|Default|GetLamp) 0 "/Game/NPCManager/EpicContent/Materials/Livingroom/M_FloorLamp_Mat_Changed.M_FloorLamp_Mat_Changed")
  ;[1 1 1] Turn light on
  (Rendering|Components|Light|SetIntensity (Variables|Default|GetPointLight) 2e+04))

(event EventBeginPlay)

(event Collision|EventActorBeginOverlap
  (params (OtherActor :type Actor%20Object%20Reference)))

(event EventTick
  (params (DeltaSeconds :type Float%20%28single-precision%29)))

(event EventFnInteract
  (params (Actor%20Reference :type Actor%20Object%20Reference))
  (Utilities|FlowControl|DoOnce false
    (:Completed
      (CallFunction|EventActivate))))

(fn ConstructionScript)