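; BP_ShowWidget is a showcase trigger actor that displays a titled path message on screen when an actor tagged Player overlaps it.
; FnShowMessage removes other BP_Path_Message widgets, then creates its own with the configured title and description, unless one is already showing.
; EventHideMessage uses a retriggerable delay of MessageTime, so repeated overlaps extend the display before the widget is removed.
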(event OnComponentBeginOverlap(Trigger)
  (params (OverlappedComponent :type Primitive%20Component%20Object%20Reference) (OtherActor :type Actor%20Object%20Reference) (OtherComp :type Primitive%20Component%20Object%20Reference) (OtherBodyIndex :type Integer) (bFromSweep :type Boolean) (SweepResult :type Hit%20Result%20Structure%20%28by%20ref%29))
  ;[1 1 1] Check that the Player is overlapping
  (if (Actor|ActorHasTag OtherActor "Player")
    ;[1 1 1] Show the message
    (CallFunction|FnShowMessage)
    ;[1 1 1] Hide the message
    (CallFunction|EventHideMessage)))

(event Custom|EventHideMessage
  ;[1 1 1] Wait MessageTime
  (Utilities|FlowControl|RetriggerableDelay (Variables|Setup|GetMessageTime))
  ;[1 1 1] Remove the widget from the screen
  (Utilities|IsValid (Variables|Default|GetWBRef)
    (:Is%20Valid
      (Widget|RemovefromParent (Variables|Default|GetWBRef))
      (Variables|Default|SetWBRef 0))))

(fn ConstructionScript)

(fn FnShowMessage
  (Utilities|FlowControl|Sequence
    (:then_0
      ;[1 1 1] Remove all the path messages, except this widget if already spawned
      (bind _foundwidgets (Widget|GetAllWidgetsOfClass "/Game/NPCManager/Blueprints/Showcase/BP_Path_Message.BP_Path_Message_C" true))
      (for _array_element _foundwidgets
        (bind _output_get (LocalVariables|SetWidget _array_element))
        (if (!= _output_get (Variables|Default|GetWBRef))
          (Widget|RemovefromParent (LocalVariables|GetWidget)))))
    (:then_1
      (Utilities|IsValid (Variables|Default|GetWBRef)
        (:Is%20Not%20Valid
          ;[1 1 1] Create a new widget class
          (bind _returnvalue (UserInterface|CreateWidget "/Game/NPCManager/Blueprints/Showcase/BP_Path_Message.BP_Path_Message_C"))
          (Utilities|IsValid _returnvalue
            (:Is%20Valid
              (Variables|Default|SetWBRef _returnvalue)
              ;[1 1 1] Set the title and description of this widget
              (Default|FnSetTitle (Variables|Default|GetWBRef) (Variables|Setup|GetMessageTitle))
              (Default|FnSetDescription (Variables|Default|GetWBRef) (Variables|Setup|GetMessageDescription))
              ;[1 1 1] Add the widget to the viewport and call function fnShowMessage
              (UserInterface|Viewport|AddtoViewport (Variables|Default|GetWBRef) 0)
              (Default|FnShowMessage (Variables|Default|GetWBRef)))))))))