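; BP_ChangeTask is a showcase trigger actor that switches an NPC's assigned task when the player enters it.
; On player overlap it finds the NPC's Comp_NPC_Controller_CustomTaskOrder component, alternates AssignedTask between two tasks with a FlipFlop, and calls EventNextTask.
; A DoOnce limits it to one switch per entry and resets when the player leaves the trigger.
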(event OnComponentBeginOverlap(Trigger)
  (params (OverlappedComponent :type Primitive%20Component%20Object%20Reference) (OtherActor :type Actor%20Object%20Reference) (OtherComp :type Primitive%20Component%20Object%20Reference) (OtherBodyIndex :type Integer) (bFromSweep :type Boolean) (SweepResult :type Hit%20Result%20Structure%20%28by%20ref%29))
  (bind _npc (Variables|Setup|GetNPC))
  (bind _returnvalue (Actor|GetComponentbyClass _npc "/Game/NPCManager/Blueprints/Characters/NPC/CustomTaskOrder/Comp_NPC_Controller_CustomTaskOrder.Comp_NPC_Controller_CustomTaskOrder_C"))
  ;[1 1 1] Check that the Player is overlapping
  (if (Actor|ActorHasTag OtherActor "Player")
    ;[1 1 1] Check that the NPC has the correct component
    (Utilities|IsValid _returnvalue
      (:Is%20Valid
        (Variables|Default|SetNPCController _returnvalue)
        (Utilities|FlowControl|DoOnce false
          (:Completed
            ;[1 1 1] Flip flop between Task 0 and 1
            (Utilities|FlowControl|FlipFlop
              (:A
                (Variables|/Game/NPCManager/Blueprints/Characters/NPC/CustomTaskOrder/Comp_NPC_Controller_CustomTaskOrder.Comp_NPC_Controller_CustomTaskOrder_C|SetAssignedTask (Variables|Default|GetNPCController) 1)
                (Default|EventNextTask (Variables|Default|GetNPCController)))
              (:B
                (Variables|/Game/NPCManager/Blueprints/Characters/NPC/CustomTaskOrder/Comp_NPC_Controller_CustomTaskOrder.Comp_NPC_Controller_CustomTaskOrder_C|SetAssignedTask (Variables|Default|GetNPCController) 0)
                (Default|EventNextTask (Variables|Default|GetNPCController))))))))))

(event OnComponentEndOverlap(Trigger)
  (params (OverlappedComponent :type Primitive%20Component%20Object%20Reference) (OtherActor :type Actor%20Object%20Reference) (OtherComp :type Primitive%20Component%20Object%20Reference) (OtherBodyIndex :type Integer))
  ;[1 1 1] Check that the Player is overlapping
  (if (Actor|ActorHasTag OtherActor "Player")
    (Utilities|FlowControl|DoOnce false) ; enters at Reset
  ))

(fn ConstructionScript)