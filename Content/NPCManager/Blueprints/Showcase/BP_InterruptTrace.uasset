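; BP_InterruptTrace is a placeable NPC Manager showcase actor that interrupts the routines of nearby NPCs.
; On BeginPlay, if Active, it waits StartDelay, then runs a single multi-sphere trace for pawns at its location.
; Each hit with a Comp_NPC_Controller receives an interrupt message carrying new profiles, a duration range and a permanent-change flag.
; The construction script sizes the InfluenceVolume sphere to match TraceRadius.
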(event EventBeginPlay
  ;[1 1 1] Check that the BP is Active
  (if (Variables|Setup|GetActive)
    ;[1 1 1] Wait the StartDelay
    (Utilities|FlowControl|Delay (Variables|Setup|GetStartDelay))
    ;[1 1 1] Do the sphere trace
    (CallFunction|FnSphereInterrupt)))

(fn ConstructionScript
  ;[1 1 1] Set the trace radius
  (Components|Sphere|SetSphereRadius (Variables|Default|GetInfluenceVolume) (Variables|Setup|GetTraceRadius) true))

(fn FnSphereInterrupt
  (bind _returnvalue (Transformation|GetActorLocation))
  ;[1 1 1] Do a multi-sphere trace for pawns
  (bind _outhits (Collision|MultiSphereTraceForObjects _returnvalue (+ _returnvalue "0, 0,0.010000") (Variables|Setup|GetTraceRadius) (Utilities|Array|MakeArray "ObjectTypeQuery3") false 0 (Variables|Setup|GetDebugType)))
  (for _array_element _outhits
    (LocalVariables|SetHitActor (.HitActor (Collision|BreakHitResult _array_element)))
    ;[1 1 1] Check that the hit actor is an NPC
    (Utilities|IsValid (Actor|GetComponentbyClass (LocalVariables|GetHitActor) "/Game/NPCManager/Blueprints/Characters/NPC/Comp_NPC_Controller.Comp_NPC_Controller_C")
      (:Is%20Valid
        ;[1 1 1] Interrupt NPC Routine
        (Class|BPINPCController|FnInterruptRoutine(Message) (Actor|GetComponentbyClass (LocalVariables|GetHitActor) "/Game/NPCManager/Blueprints/Characters/NPC/Comp_NPC_Controller.Comp_NPC_Controller_C") (Variables|Setup|GetNewProfiles) (Variables|Setup|GetDuration) (Variables|Setup|GetPermanentChange?))))))