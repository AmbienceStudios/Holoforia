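; BP_StreamLevel is a trigger volume that streams levels in and out when an actor tagged Player overlaps it.
; On overlap it loads LoadLevel asynchronously and visible, then after DespawnDelay unloads each level in UnloadLevels without blocking.
; Both paths skip "None" names and check the current loaded state first.
; The construction script sizes the trigger from TriggerScale.
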(event OnComponentBeginOverlap(Trigger)
  (params (OverlappedComponent :type Primitive%20Component%20Object%20Reference) (OtherActor :type Actor%20Object%20Reference) (OtherComp :type Primitive%20Component%20Object%20Reference) (OtherBodyIndex :type Integer) (bFromSweep :type Boolean) (SweepResult :type Hit%20Result%20Structure%20%28by%20ref%29))
  (if (Actor|ActorHasTag OtherActor "Player")
    (CallFunction|EventLoadLevel)
    (CallFunction|EventUnloadLevels)))

(event EventBeginPlay)

(event Collision|EventActorBeginOverlap
  (params (OtherActor :type Actor%20Object%20Reference)))

(event EventTick
  (params (DeltaSeconds :type Float%20%28single-precision%29)))

(fn ConstructionScript
  (Transformation|SetWorldScale3D (Variables|Default|GetTrigger) (Variables|Setup|GetTriggerScale)))

(event Custom|EventLoadLevel
  (bind _loadlevel (Variables|Setup|GetLoadLevel))
  (if (and (Utilities|Name|NotEqual(Name) _loadlevel "None") (not (Class|LevelStreaming|IsLevelLoaded (Class|GameplayStatics|GetStreamingLevel _loadlevel))))
    (Game|LoadStreamLevel(byName) (Variables|Setup|GetLoadLevel) true)))

(event Custom|EventUnloadLevels
  (Utilities|FlowControl|Delay (Variables|Setup|GetDespawnDelay))
  (for _array_element (Variables|Setup|GetUnloadLevels)
    (bind _output_get (Variables|Default|SetUnloadLevel _array_element))
    (if (and (Utilities|Name|NotEqual(Name) _output_get "None") (Class|LevelStreaming|IsLevelLoaded (Class|GameplayStatics|GetStreamingLevel _output_get)))
      (Game|UnloadStreamLevel(byName) (Variables|Default|GetUnloadLevel) false))))