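; BP_Projectile is a projectile Blueprint under the player character folder that damages what it hits.
; The construction script sets the movement component's velocity from ProjectileVelocity, and BeginPlay makes the collision sphere ignore the player pawn when moving.
; On hit, it applies BaseDamage with OwnerActor as causer, adds ProjectileVelocity as force to its own sphere, then destroys itself after a short delay.
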(event OnComponentHit(Sphere)
  (params (HitComponent :type Primitive%20Component%20Object%20Reference) (OtherActor :type Actor%20Object%20Reference) (OtherComp :type Primitive%20Component%20Object%20Reference) (NormalImpulse :type Vector :default "0, 0, 0") (Hit :type Hit%20Result%20Structure%20%28by%20ref%29))
  ;[1 1 1] Apply damage
  (Game|Damage|ApplyDamage OtherActor (Variables|Default|GetBaseDamage) 0 (Variables|Default|GetOwnerActor))
  ;[1 1 1] Add force
  (Physics|AddForce (Variables|Default|GetSphere) (Variables|Default|GetProjectileVelocity) "None" false)
  ;[1 1 1] Add a small delay and Destroy the projectile
  (Utilities|FlowControl|Delay 0.2)
  (Actor|DestroyActor))

(event EventBeginPlay
  ;[1 1 1] Ignore the Player
  (Collision|IgnoreActorwhenMoving (Variables|Default|GetSphere) (Game|Player|GetPlayerPawn 0) true))

(fn ConstructionScript
  ;[1 1 1] Set velocity
  (Variables|/Script/Engine.MovementComponent|SetVelocity (Variables|Default|GetProjectileMovement) (Variables|Default|GetProjectileVelocity)))