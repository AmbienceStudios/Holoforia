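; BP_SplineCrowd_Intersection is a trigger that lets spline crowd NPCs randomly switch paths where crowd routes meet.
; On overlap by a Character tagged SplineCrowd, it rolls against a clamped switch chance and requires at least two listed paths.
; It removes the NPC from its current path's NPC list and adds it to a random other path's list.
; The construction script applies trigger scale and visibility settings.
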(event OnComponentBeginOverlap(Trigger)
  (params (OverlappedComponent :type Primitive%20Component%20Object%20Reference) (OtherActor :type Actor%20Object%20Reference) (OtherComp :type Primitive%20Component%20Object%20Reference) (OtherBodyIndex :type Integer) (bFromSweep :type Boolean) (SweepResult :type Hit%20Result%20Structure%20%28by%20ref%29))
  ;[1 1 1] Check the overlapped actor is part of a spline crowd
  (if (Actor|ActorHasTag OtherActor "SplineCrowd")
    (bind _ascharacter (Utilities|Casting|CastToCharacter OtherActor))
    (Variables|Default|SetOverlappedActor _ascharacter)
    ;[1 1 1] Change NPC path
    (CallFunction|FnChangePaths)))

(event EventBeginPlay)

(fn ConstructionScript
  ;[1 1 1] Set trigger scale and visibility
  (Transformation|SetWorldScale3D (Variables|Default|GetTrigger) (Variables|Setup|GetTriggerScale))
  (Rendering|SetVisibility (Variables|Default|GetTrigger) (Variables|Setup|GetTriggerVisible) false)
  (Development|SetHiddeninGame (Variables|Default|GetTrigger) (Variables|Setup|GetTriggerHidden) false))

(fn FnChangePaths
  ;[1 1 1] Check percent chance to change paths
  (if (>= (Math|Float|Clamp(Float) (Variables|Setup|GetPercentChanceToSwitch)) (Math|Random|RandomFloatinRange 0.0 1.0))
    ;[1 1 1] Set the Temp List and check that we have at least 2 paths
    (bind _output_get (LocalVariables|SetTempList (Variables|Setup|GetSplinePathList)))
    (if (>= (Utilities|Array|Length _output_get) 2)
      ;[1 1 1] Loop through all the paths
      (bind (_array_element _array_index) (Utilities|Array|ForEachLoopwithBreak (LocalVariables|GetTempList))
        (:LoopBody
          (LocalVariables|SetPath _array_element)
          (LocalVariables|SetIndex _array_index)
          ;[1 1 1] Is this actor part of this Path?
          (if (Utilities|Array|ContainsItem (Variables|/Game/NPCManager/Blueprints/Characters/NPC/Crowds/SplineCrowd/BP_SplineCrowd.BP_SplineCrowd_C|GetNPCList (LocalVariables|GetPath)) (Variables|Default|GetOverlappedActor))
            ;[1 1 1] Remove this actor from the NPC List
            (Utilities|Array|RemoveItem (Variables|/Game/NPCManager/Blueprints/Characters/NPC/Crowds/SplineCrowd/BP_SplineCrowd.BP_SplineCrowd_C|GetNPCList (LocalVariables|GetPath)) (Variables|Default|GetOverlappedActor))
            ;[1 1 1] Remove this Path from the temp list
            (Utilities|Array|RemoveItem (LocalVariables|GetTempList) (LocalVariables|GetPath))))
        (:Completed
          ;[1 1 1] Add Overlapped Actor to a random path, other than its original one
          (Utilities|Array|Add (Variables|/Game/NPCManager/Blueprints/Characters/NPC/Crowds/SplineCrowd/BP_SplineCrowd.BP_SplineCrowd_C|GetNPCList (Utilities|Array|Get(acopy) (LocalVariables|GetTempList) (Math|Random|RandomIntegerinRange 0 (Utilities|Array|LastIndex (LocalVariables|GetTempList))))) (Variables|Default|GetOverlappedActor)))))))