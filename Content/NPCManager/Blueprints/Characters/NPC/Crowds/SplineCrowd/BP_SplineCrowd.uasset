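; Spline-based crowd spawner that scatters random NPCs along a spline and keeps them walking along it.
; NPCs follow the spline direction, steering back when off-path, and teleport to the start on open splines.
; Single Player uses movement input on Tick; Multiplayer sends Blackboard targets to AI controllers on an authority timer.
; An optional trigger spawns and shows NPCs for players, hiding and pausing them when none remain.
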(event OnComponentBeginOverlap(Trigger)
  (params (OverlappedComponent :type Primitive%20Component%20Object%20Reference) (OtherActor :type Actor%20Object%20Reference) (OtherComp :type Primitive%20Component%20Object%20Reference) (OtherBodyIndex :type Integer) (bFromSweep :type Boolean) (SweepResult :type Hit%20Result%20Structure%20%28by%20ref%29))
  ;[1 1 1] Check that the Player overlapped
  (if (and (Actor|ActorHasTag OtherActor "Player") (Variables|Setup|GetUseTrigger))
    (Networking|SwitchHasAuthority
      (:Authority
        ;[1 1 1] If NPCs have not spawned, spawn them
        (if (Variables|Default|GetSpawnedNPCs)
          _
          (else
            (CallFunction|FnSpawnNPCs)
            (Utilities|FlowControl|Delay 0.2)
            (CallFunction|EventMoveNPCs)))
        ;[1 1 1] Move NPCs and enable the NPCs
        (Variables|Default|SetMoveNPCs true)
        (CallFunction|EventEnableNPCs true)))))

(event OnComponentEndOverlap(Trigger)
  (params (OverlappedComponent :type Primitive%20Component%20Object%20Reference) (OtherActor :type Actor%20Object%20Reference) (OtherComp :type Primitive%20Component%20Object%20Reference) (OtherBodyIndex :type Integer))
  ;[1 1 1] Check that the Player overlapped
  (if (and (Actor|ActorHasTag OtherActor "Player") (Variables|Setup|GetUseTrigger))
    (Networking|SwitchHasAuthority
      (:Authority
        (Utilities|FlowControl|Delay 2.0)
        ;[1 1 1] Check that there are Players around
        (bind _found_player (CallFunction|FnTraceforPlayers))
        (if (not _found_player)
          ;[1 1 1] Stop moving NPCs and disable the NPCs
          (Variables|Default|SetMoveNPCs false)
          (CallFunction|EventEnableNPCs false))))))

(event EventBeginPlay
  ;[1 1 1] Check that this BP is Active
  (if (Variables|Setup|GetActive)
    (Networking|SwitchHasAuthority
      (:Authority
        ;[1 1 1] Set the NPC Tag
        (Variables|Default|SetNPCTag (Utilities|String|StringToName (Utilities|GetDisplayName self)))
        ;[1 1 1] Check we are not not using the Trigger
        (if (not (Variables|Setup|GetUseTrigger))
          ;[1 1 1] Wait a random time
          (Utilities|FlowControl|Delay (Math|Random|RandomFloatinRange 0.0 0.75))
          (Utilities|FlowControl|Sequence
            (:then_0
              ;[1 1 1] Check that we have not spawned NPCs
              (if (not (Variables|Default|GetSpawnedNPCs))
                ;[1 1 1] Spawn NPCs
                (CallFunction|FnSpawnNPCs)
                ;[1 1 1] If we use the trigger, disable the NPCs
                (if (Variables|Setup|GetUseTrigger)
                  (bind _found_player (CallFunction|FnTraceforPlayers))
                  (if (not _found_player)
                    (Variables|Default|SetMoveNPCs false)
                    (CallFunction|FnEnableNPCs false)))))
            (:then_1
              (switch Utilities|FlowControl|Switch|SwitchonEnum_SplineCrowdMode (Variables|Setup|GetMode)
                (:NewEnumerator1
                  (CallFunction|EventMoveNPCs))))))))))

(event EventTick
  (params (DeltaSeconds :type Float%20%28single-precision%29))
  (switch Utilities|FlowControl|Switch|SwitchonEnum_SplineCrowdMode (Variables|Setup|GetMode)
    (:NewEnumerator0
      ;[1 1 1] Check if we can Move the NPCs and move them
      (if (Variables|Default|GetMoveNPCs)
        (CallFunction|FnMoveNPCs)))))

(fn ConstructionScript
  ;[1 1 1] Set Closed Loop
  (Spline|SetClosedLoop (Variables|Default|GetSpline) (Variables|Setup|GetClosedLoop) true))

(fn FnSpawnNPCs
  (bind _npcclasses (Variables|Setup|GetNPCClasses))
  (bind _speedmultiplierrange (Variables|Setup|GetSpeedMultiplierRange))
  (for _index (range 0 (- (Variables|Setup|GetTotalSpawns) 1))
    ;[1 1 1] Get random distance
    (Variables|Default|SetRandomDistance (Math|Random|RandomFloatinRange 0.0 (Spline|GetSplineLength (Variables|Default|GetSpline))))
    ;[1 1 1] Spawn a random NPC
    (bind _returnvalue (Game|SpawnActorfromClass (Utilities|Array|Get(acopy) _npcclasses (Math|Random|RandomIntegerinRange 0 (Utilities|Array|LastIndex _npcclasses))) (|GETRANDOMLOCATIONANDROTATION) "AdjustIfPossibleButAlwaysSpawn" 0 0))
    (LocalVariables|SetSpawnedNPC _returnvalue)
    (switch Utilities|FlowControl|Switch|SwitchonEnum_SplineCrowdMode (Variables|Setup|GetMode)
      (:NewEnumerator0
        _)
      (:NewEnumerator1
        (bind _asbp_spline_npc_controller (Utilities|Casting|CastToBP_SplineNPC_Controller (AI|GetAIController (LocalVariables|GetSpawnedNPC))))
        (Default|EventRunBT _asbp_spline_npc_controller)))
    ;[1 1 1] Add  Self tag
    (Utilities|Array|Add (Variables|/Script/Engine.Actor|GetTags (LocalVariables|GetSpawnedNPC)) (Variables|Default|GetNPCTag))
    ;[1 1 1] Add  spline crowd tag
    (Utilities|Array|Add (Variables|/Script/Engine.Actor|GetTags (LocalVariables|GetSpawnedNPC)) "SplineCrowd")
    ;[1 1 1] Force mesh LOD
    (Components|SkinnedMesh|SetForcedLOD (Variables|/Script/Engine.Character|GetMesh (LocalVariables|GetSpawnedNPC)) (Variables|Setup|GetMeshForcedLOD))
    ;[1 1 1] Set a random walking speed
    (Variables|/Script/Engine.CharacterMovementComponent|SetMaxWalkSpeed (Variables|/Script/Engine.Character|GetCharacterMovement (LocalVariables|GetSpawnedNPC)) (* (Variables|/Script/Engine.CharacterMovementComponent|GetMaxWalkSpeed (Variables|/Script/Engine.Character|GetCharacterMovement (LocalVariables|GetSpawnedNPC))) (Math|Random|RandomFloatinRange (.x _speedmultiplierrange) (.y _speedmultiplierrange))))
    ;[1 1 1] Add NPC to the NPC List
    (Utilities|Array|Add (Variables|Setup|GetNPCList) (LocalVariables|GetSpawnedNPC)))
  (Variables|Default|SetMoveNPCs true)
  (Variables|Default|SetSpawnedNPCs true))

(fn FnMoveNPCs
  (bind _splineoffsetrange (Variables|Setup|GetSplineOffsetRange))
  (bind _spline (Variables|Default|GetSpline))
  ;[1 1 1] Loop through all NPCs
  (for _array_element (Variables|Setup|GetNPCList)
    (bind _output_get (LocalVariables|SetNPC _array_element))
    (Utilities|IsValid _output_get
      (:Is%20Valid
        (Utilities|IsValid (Actor|GetComponentbyClass (LocalVariables|GetNPC) "/Game/NPCManager/Blueprints/Characters/NPC/Crowds/SplineCrowd/Comp_SplineNPC.Comp_SplineNPC_C")
          (:Is%20Valid
            (LocalVariables|SetNPCComp (Actor|GetComponentbyClass (LocalVariables|GetNPC) "/Game/NPCManager/Blueprints/Characters/NPC/Crowds/SplineCrowd/Comp_SplineNPC.Comp_SplineNPC_C"))
            ;[1 1 1] Check if the NPC distance to the spline is less than or equal to the offset range
            (if (<= (Math|Vector|Distance2D(Vector) (Transformation|GetActorLocation (LocalVariables|GetNPC)) (Spline|FindLocationClosesttoWorldLocation (Variables|Default|GetSpline) (Transformation|GetActorLocation (LocalVariables|GetNPC)) "World")) (select (< (.x _splineoffsetrange) (.y _splineoffsetrange)) (.y _splineoffsetrange) (.x _splineoffsetrange)))
              ;[1 1 1] Calculate Direction
              (LocalVariables|SetDirection (Math|Vector|GetForwardVector (Class|SplineComponent|FindRotationClosesttoWorldLocation (Variables|Default|GetSpline) (Transformation|GetActorLocation (LocalVariables|GetNPC)) "World")))
              (switch Utilities|FlowControl|Switch|SwitchonEnum_SplineCrowdMode (Variables|Setup|GetMode)
                (:NewEnumerator0
                  ;[1 1 1] Add movement input along spline
                  (Pawn|Input|AddMovementInput (LocalVariables|GetNPC) (LocalVariables|GetDirection) 1.0 false))
                (:NewEnumerator1
                  (AI|Components|Blackboard|SetValueasVector (AI|GetBlackboard (LocalVariables|GetNPC)) (Utilities|Name|MakeLiteralName "Location") (+ (Transformation|GetActorLocation (LocalVariables|GetNPC)) (* (LocalVariables|GetDirection) 5e+02)))))
              (else
                ;[1 1 1] Calculate Direction
                (LocalVariables|SetDirection (Math|Vector|GetForwardVector (Math|Rotator|FindLookatRotation (Transformation|GetActorLocation (LocalVariables|GetNPC)) (Spline|FindLocationClosesttoWorldLocation (Variables|Default|GetSpline) (Transformation|GetActorLocation (LocalVariables|GetNPC)) "World"))))
                (switch Utilities|FlowControl|Switch|SwitchonEnum_SplineCrowdMode (Variables|Setup|GetMode)
                  (:NewEnumerator0
                    ;[1 1 1] Add movement input towards spline
                    (Pawn|Input|AddMovementInput (LocalVariables|GetNPC) (LocalVariables|GetDirection) 1.0 false))
                  (:NewEnumerator1
                    (AI|Components|Blackboard|SetValueasVector (AI|GetBlackboard (LocalVariables|GetNPC)) (Utilities|Name|MakeLiteralName "Location") (+ (Transformation|GetActorLocation (LocalVariables|GetNPC)) (* (LocalVariables|GetDirection) 5e+02)))))))
            ;[1 1 1] Check the NPC is moving (not stuck)
            (if (>= (Math|Vector|VectorLength (Variables|/Script/Engine.MovementComponent|GetVelocity (Variables|/Script/Engine.Character|GetCharacterMovement (LocalVariables|GetNPC)))) 1.0)
              _
              (else
                (Default|EventChangeCollision (LocalVariables|GetNPCComp))))
            ;[1 1 1] Check that this is NOT a closed loop
            (if (not (Variables|Setup|GetClosedLoop))
              ;[1 1 1] Check the distance between the NPC and the last spline point. Is it less than or equal to the Teleport Distance?
              (if (<= (Math|Vector|Distance2D(Vector) (Transformation|GetActorLocation (LocalVariables|GetNPC)) (Spline|GetLocationatSplinePoint _spline (- (Spline|GetNumberOfSplinePoints _spline) 1) "World")) (Variables|Setup|GetTeleportDistance))
                ;[1 1 1] Teleport NPC
                (CallFunction|EventServerTeleportNPC (LocalVariables|GetNPC))))))))))

(fn FnTeleportNPC
  (params (NPC%20to%20teleport :type Actor%20Object%20Reference))
  (bind _spline (Variables|Default|GetSpline))
  (bind _splineoffsetrange (Variables|Setup|GetSplineOffsetRange))
  (bind _returnvalue (Spline|GetRotationatSplinePoint _spline 0 "World"))
  (bind _output_get (LocalVariables|SetNPC NPC%20to%20teleport))
  (LocalVariables|SetLocation (Transformation|GetActorLocation _output_get))
  ;[1 1 1] Teleport the NPC to the beginning of the spline and give it a random offset
  (Transformation|SetActorLocationAndRotation (LocalVariables|GetNPC) (+ (+ (+ (Spline|GetLocationatSplinePoint _spline 0 "World") (* (Math|Vector|GetForwardVector _returnvalue) (Math|Random|RandomFloatinRange 1.0 (* (.y _splineoffsetrange) 2.0)))) (* (Math|Vector|GetRightVector _returnvalue) (Math|Random|RandomFloatinRange (.x _splineoffsetrange) (.y _splineoffsetrange)))) "0, 0,100.000000") _returnvalue false true))

(fn FnEnableNPCs
  (params (Enable :type Boolean))
  (if Enable
    (for _array_element (Variables|Setup|GetNPCList)
      (LocalVariables|SetNPC _array_element)
      ;[1 1 1] Show NPC and enable collision
      (Rendering|SetActorHiddenInGame (LocalVariables|GetNPC) false)
      (Collision|SetActorEnableCollision (LocalVariables|GetNPC) true))
    (else
      (for _array_element_2 (Variables|Setup|GetNPCList)
        (LocalVariables|SetNPC _array_element_2)
        ;[1 1 1] Hide NPC and disable collision
        (Rendering|SetActorHiddenInGame (LocalVariables|GetNPC) true)
        (Collision|SetActorEnableCollision (LocalVariables|GetNPC) false)))))

(fn FnTraceforPlayers
  (bind _trigger (Variables|Default|GetTrigger))
  (bind _returnvalue (Transformation|GetWorldLocation _trigger))
  ;[1 1 1] Trace for nearby Pawns
  (bind (_outhits _returnvalue_2) (Class|KismetSystemLibrary|BoxTraceMultiforObjects _returnvalue (+ _returnvalue "0, 0,0.010000") (.BoxExtent (Collision|GetComponentBounds _trigger)) (Variables|/Script/Engine.SceneComponent|GetRelativeRotation _trigger) (Utilities|Array|MakeArray "ObjectTypeQuery3") false 0 "None" true))
  ;[1 1 1] Check if we hit a pawn with the tag "Player"
  (if _returnvalue_2
    (bind _array_element (Utilities|Array|ForEachLoopwithBreak _outhits :!label _label)
      (:LoopBody
        (if (Actor|ActorHasTag (.HitActor (Collision|BreakHitResult _array_element)) "Player")
          (LocalVariables|SetFound true)
          (goto _label Break)))
      (:Completed
        (return (LocalVariables|GetFound))))
    (else
      (return (LocalVariables|GetFound)))))

(event Custom|EventServerTeleportNPC
  (params (NPC :type Actor%20Object%20Reference))
  (bind _spline (Variables|Default|GetSpline))
  (bind _splineoffsetrange (Variables|Setup|GetSplineOffsetRange))
  (bind _returnvalue (Spline|GetRotationatSplinePoint _spline 0 "World"))
  (Variables|Default|SetNPCActor NPC)
  ;[1 1 1] Calculate the NPC's Target Location
  (Variables|Default|SetTargetLocation (+ (+ (+ (Spline|GetLocationatSplinePoint _spline 0 "World") (* (Math|Vector|GetForwardVector _returnvalue) (Math|Random|RandomFloatinRange 1.0 (* (.y _splineoffsetrange) 2.0)))) (* (Math|Vector|GetRightVector _returnvalue) (Math|Random|RandomFloatinRange (.x _splineoffsetrange) (.y _splineoffsetrange)))) "0, 0,100.000000"))
  (CallFunction|EventMCTeleportNPC (Variables|Default|GetNPCActor)))

(event Custom|EventMCTeleportNPC
  (params (NPC :type Actor%20Object%20Reference))
  (Transformation|SetActorLocationAndRotation NPC (Variables|Default|GetTargetLocation) (Spline|GetRotationatSplinePoint (Variables|Default|GetSpline) 0 "World") false true))

(event Custom|EventMoveNPCs
  (Utilities|Time|SetTimerbyEvent (delegate Custom|EventMoveNPCs) 1.0 true)
  (Networking|SwitchHasAuthority
    (:Authority
      ;[1 1 1] Check if we can Move the NPCs and move them
      (if (Variables|Default|GetMoveNPCs)
        (CallFunction|FnMoveNPCs)))))

(event Custom|EventEnableNPCs
  (params (Enable :type Boolean))
  (CallFunction|FnEnableNPCs Enable))