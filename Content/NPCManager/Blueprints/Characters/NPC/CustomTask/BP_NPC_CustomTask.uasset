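; NPC character Blueprint that handles trigger-based interactions, a floating name/HP HUD and physical animation, using Comp_NPC_Controller for NPC data.
; Trigger overlaps message BPI_NPC_Interaction actors, with a delayed controller re-check, and initiate interaction with other NPCs.
; If enabled, a timer refreshes the HUD from the controller, hiding it at zero HP, while Tick yaws it toward the camera.
; BeginPlay also enables physics-blended animation below a chosen bone.
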(event OnComponentBeginOverlap(Interaction_Trigger)
  (params (OverlappedComponent :type Primitive%20Component%20Object%20Reference) (OtherActor :type Actor%20Object%20Reference) (OtherComp :type Primitive%20Component%20Object%20Reference) (OtherBodyIndex :type Integer) (bFromSweep :type Boolean) (SweepResult :type Hit%20Result%20Structure%20%28by%20ref%29))
  (Variables|Default|SetOverlappedActor OtherActor)
  (Utilities|FlowControl|Sequence
    (:then_0
      ;[1 1 1] Does this actor implement the Interaction BPI?
      (if (Utilities|DoesObjectImplementInterface (Variables|Default|GetOverlappedActor) "/Game/NPCManager/Blueprints/Core/Interfaces/BPI_NPC_Interaction.BPI_NPC_Interaction_C")
        ;[1 1 1] Interact with object
        (Class|BPINPCInteraction|FnInteract(Message) (Variables|Default|GetOverlappedActor) self)
        (CallFunction|EventCheckInteractionObject)))
    (:then_1
      ;[1 1 1] Is this an NPC?
      (Utilities|IsValid (Actor|GetComponentbyClass (Variables|Default|GetOverlappedActor) "/Game/NPCManager/Blueprints/Characters/NPC/Comp_NPC_Controller.Comp_NPC_Controller_C")
        (:Is%20Valid
          (Variables|Default|SetNPCController (Actor|GetComponentbyClass (Variables|Default|GetOverlappedActor) "/Game/NPCManager/Blueprints/Characters/NPC/Comp_NPC_Controller.Comp_NPC_Controller_C"))
          ;[1 1 1] Initiate interaction with the overlapped NPC
          (Class|BPINPCInteraction|FnInitInteraction(Message) (Variables|Default|GetNPCController) self))))))

(event EventBeginPlay
  (Utilities|FlowControl|Sequence
    (:then_0
      (|UPDATEHUD))
    (:then_1
      (|SETPHYSICALANIMATION))))

(event EventTick
  (params (DeltaSeconds :type Float%20%28single-precision%29))
  (|ROTATEHUD))

(fn ConstructionScript)

(event Custom|EventCheckInteractionObject
  (bind _returnvalue (Actor|GetComponentbyClass "/Game/NPCManager/Blueprints/Characters/NPC/Comp_NPC_Controller.Comp_NPC_Controller_C"))
  ;[1 1 1] Wait 2 seconds
  (Utilities|FlowControl|Delay 2.0)
  ;[1 1 1] See if NPC is still near the object and interact again
  (Utilities|IsValid _returnvalue
    (:Is%20Valid
      (Default|FnCheckInteraction _returnvalue (.BoxExtent (Collision|GetComponentBounds (Variables|Default|GetInteraction_Trigger)))))))

(event Custom|EventUpdateHUD
  (bind _returnvalue (Utilities|Time|SetTimerbyEvent (delegate Custom|EventUpdateHUD) 0.25 true))
  (Variables|Default|SetHUDHandler _returnvalue)
  (CallFunction|EventSetHUD))

(event Custom|EventSetHUD
  (bind _returnvalue (Actor|GetComponentbyClass "/Game/NPCManager/Blueprints/Characters/NPC/Comp_NPC_Controller.Comp_NPC_Controller_C"))
  (bind _generalsettings (Variables|/Game/NPCManager/Blueprints/Characters/NPC/Comp_NPC_Controller.Comp_NPC_Controller_C|GetGeneralSettings _returnvalue))
  (bind (_npcname _pickrandomname _datatablewithnames _totalhp) (Utilities|Struct|BreakStruct_NPC_GeneralInfo _generalsettings))
  (bind _aswbp_npc_hud (Utilities|Casting|CastToWBP_NPC_HUD (UserInterface|GetUserWidgetObject (Variables|Default|GetHUD))))
  (Variables|Default|SetHUDRef _aswbp_npc_hud)
  ;[1 1 1] Set Name and HP in the HUD
  (Utilities|FlowControl|Sequence
    (:then_0
      (Default|FnSetName (Variables|Default|GetHUDRef) _npcname))
    (:then_1
      (Default|FnSetHP (Variables|Default|GetHUDRef) (Variables|/Game/NPCManager/Blueprints/Characters/NPC/Comp_NPC_Controller.Comp_NPC_Controller_C|GetCurrentHP _returnvalue) _totalhp))
    (:then_2
      (if (== (Variables|/Game/NPCManager/Blueprints/Characters/NPC/Comp_NPC_Controller.Comp_NPC_Controller_C|GetCurrentHP _returnvalue) 0.0)
        (Default|FnHideHUD (Variables|Default|GetHUDRef))))))