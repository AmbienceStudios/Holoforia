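; Base swinging door that NPCs open through an interact event and that closes automatically once they leave.
; Front and back triggers record which side an NPC arrived from, setting the swing direction for the timeline-driven rotation.
; Door collision turns off once fully open and returns once closed.
; On trigger exit, box traces recheck both sides every second until no pawns remain, then it closes after a delay.
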(event OnComponentBeginOverlap(TriggerFront)
  (params (OverlappedComponent :type Primitive%20Component%20Object%20Reference) (OtherActor :type Actor%20Object%20Reference) (OtherComp :type Primitive%20Component%20Object%20Reference) (OtherBodyIndex :type Integer) (bFromSweep :type Boolean) (SweepResult :type Hit%20Result%20Structure%20%28by%20ref%29))
  ;[1 1 1] Check this is an NPC
  (if (Actor|ActorHasTag OtherActor "NPC")
    ;[1 1 1] Check that no one is here
    (if (not (Variables|Default|GetSomeoneHere))
      (Variables|Default|SetFrontTrigger true)
      (Variables|Default|SetBackTrigger false)
      (Variables|Default|SetSomeoneHere true))))

(event OnComponentEndOverlap(TriggerFront)
  (params (OverlappedComponent :type Primitive%20Component%20Object%20Reference) (OtherActor :type Actor%20Object%20Reference) (OtherComp :type Primitive%20Component%20Object%20Reference) (OtherBodyIndex :type Integer))
  ;[1 1 1] Check this is an NPC
  (if (Actor|ActorHasTag OtherActor "NPC")
    ;[1 1 1] Close the front door
    (CallFunction|EventCheckandClose true)))

(event OnComponentBeginOverlap(TriggerBack)
  (params (OverlappedComponent :type Primitive%20Component%20Object%20Reference) (OtherActor :type Actor%20Object%20Reference) (OtherComp :type Primitive%20Component%20Object%20Reference) (OtherBodyIndex :type Integer) (bFromSweep :type Boolean) (SweepResult :type Hit%20Result%20Structure%20%28by%20ref%29))
  ;[1 1 1] Check this is an NPC
  (if (Actor|ActorHasTag OtherActor "NPC")
    ;[1 1 1] Check that no one is here
    (if (not (Variables|Default|GetSomeoneHere))
      (Variables|Default|SetBackTrigger true)
      (Variables|Default|SetFrontTrigger false)
      (Variables|Default|SetSomeoneHere true))))

(event OnComponentEndOverlap(TriggerBack)
  (params (OverlappedComponent :type Primitive%20Component%20Object%20Reference) (OtherActor :type Actor%20Object%20Reference) (OtherComp :type Primitive%20Component%20Object%20Reference) (OtherBodyIndex :type Integer))
  ;[1 1 1] Check this is an NPC
  (if (Actor|ActorHasTag OtherActor "NPC")
    ;[1 1 1] Close the back door
    (CallFunction|EventCheckandClose false)))

(fn ConstructionScript)

(fn FnCheckforActors
  (bind _triggerfront (Variables|Default|GetTriggerFront))
  (bind _triggerback (Variables|Default|GetTriggerBack))
  (bind _returnvalue (Transformation|GetWorldLocation _triggerback))
  (bind _returnvalue_2 (Transformation|GetWorldLocation _triggerfront))
  (Utilities|FlowControl|Sequence
    (:then_0
      (Utilities|FlowControl|Sequence
        (:then_0
          ;[1 1 1] Trace the front
          (bind _returnvalue_3 (Class|KismetSystemLibrary|BoxTraceSingleforObjects _returnvalue_2 (+ _returnvalue_2 "0, 0,0.010000") (.BoxExtent (Collision|GetComponentBounds _triggerfront)) (Transformation|GetWorldRotation _triggerfront) (Utilities|Array|MakeArray "ObjectTypeQuery3") false 0 (select (Variables|Setup|GetDebugClosingTrace) "ForDuration" "None") true))
          (LocalVariables|SetSomethingFound _returnvalue_3))
        (:then_1
          (if (not (LocalVariables|GetSomethingFound))
            ;[1 1 1] Trace the back
            (bind _returnvalue_4 (Class|KismetSystemLibrary|BoxTraceSingleforObjects _returnvalue (+ _returnvalue "0, 0,0.010000") (.BoxExtent (Collision|GetComponentBounds _triggerback)) (Transformation|GetWorldRotation _triggerback) (Utilities|Array|MakeArray "ObjectTypeQuery3") false 0 (select (Variables|Setup|GetDebugClosingTrace) "ForDuration" "None") true))
            (LocalVariables|SetSomethingFound _returnvalue_4)))))
    (:then_1
      (return (LocalVariables|GetSomethingFound)))))

(event Custom|EventOpenDoor
  ;[1 1 1] Check that we can open the door and are not already opening it
  (if (and (Variables|Default|GetCanOpen) (not (Variables|Default|GetOpening)))
    ;[1 1 1] Set goal rotation
    (if (Variables|Default|GetFrontTrigger)
      (Variables|Default|SetGoalRotation -9e+01)
      ;[1 1 1] Open the door and set the parameters
      (bind _alpha (Timeline|TM_Open PlayFromStart)
        (:Update
          (Transformation|SetRelativeRotation (Variables|Default|GetDoor) (Math|Rotator|MakeRotator 0.0 0.0 (Math|Float|Lerp 0.0 (Variables|Default|GetGoalRotation) _alpha)) false false)
          (Variables|Default|SetOpening true))
        (:Finished
          (Variables|Default|SetCanClose true)
          (Variables|Default|SetCanOpen false)
          (Variables|Default|SetOpening false)
          ;[1 1 1] Disable Door Collision
          (Collision|SetCollisionEnabled (Variables|Default|GetDoor) "NoCollision")))
      (elif (Variables|Default|GetBackTrigger)
        (Variables|Default|SetGoalRotation 9e+01)
        (Timeline|TM_Open PlayFromStart)))))

(event Custom|EventCloseDoor
  ;[1 1 1] Check that we can close the door and are not already closing it
  (if (and (Variables|Default|GetCanClose) (not (Variables|Default|GetClosing)))
    ;[1 1 1] Check that we can close the door
    (if (and (not (Variables|Default|GetFrontTrigger)) (not (Variables|Default|GetBackTrigger)))
      ;[1 1 1] Close the door and set t he parameters
      (bind _alpha (Timeline|TM_Close PlayFromStart)
        (:Update
          (Transformation|SetRelativeRotation (Variables|Default|GetDoor) (Math|Rotator|MakeRotator 0.0 0.0 (Math|Float|Lerp (Variables|Default|GetGoalRotation) 0.0 _alpha)) false false)
          (Variables|Default|SetClosing true))
        (:Finished
          (Variables|Default|SetCanOpen true)
          (Variables|Default|SetCanClose false)
          (Variables|Default|SetClosing false)
          ;[1 1 1] Enable Door Collision
          (Collision|SetCollisionEnabled (Variables|Default|GetDoor) "QueryAndPhysics"))))))

(event EventFnInteract
  (params (Actor%20Reference :type Actor%20Object%20Reference))
  (Variables|Default|SetOwnerActor Actor%20Reference)
  ;[1 1 1] Check that we can interact
  (if (Variables|Setup|GetCanInteract)
    ;[1 1 1] Open the door
    (CallFunction|EventOpenDoor)))

(event Custom|EventCheckAndClose
  (params (Front :type Boolean))
  (if Front
    ;[1 1 1] Check for nearby actors
    (if (not (CallFunction|FnCheckforActors))
      (Variables|Default|SetFrontTrigger false)
      (Variables|Default|SetSomeoneHere false)
      (Utilities|FlowControl|Delay (Variables|Setup|GetOpenDuration))
      (CallFunction|EventCloseDoor)
      (else
        (Utilities|FlowControl|Delay 1.0)
        (CallFunction|EventCheckandClose true)))
    (else
      ;[1 1 1] Check for nearby actors
      (if (not (CallFunction|FnCheckforActors))
        (Variables|Default|SetBackTrigger false)
        (Variables|Default|SetSomeoneHere false)
        (Utilities|FlowControl|Delay (Variables|Setup|GetOpenDuration))
        (CallFunction|EventCloseDoor)
        (else
          (Utilities|FlowControl|Delay 1.0)
          (CallFunction|EventCheckandClose false))))))