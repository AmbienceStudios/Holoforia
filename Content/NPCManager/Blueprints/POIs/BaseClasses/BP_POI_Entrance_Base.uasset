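; Base Blueprint for a point-of-interest entrance that tells NPCs when they reach their POI.
; When an actor overlaps the Trigger, it looks for an NPC Controller component and, if that component implements BPI_NPC_Controller, sends it an arrived-at-POI message with the parent POI.
; The construction script sets the Entrance component's editor visibility and in-game hiding from exposed flags.
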(event OnComponentBeginOverlap(Trigger)
  (params (OverlappedComponent :type Primitive%20Component%20Object%20Reference) (OtherActor :type Actor%20Object%20Reference) (OtherComp :type Primitive%20Component%20Object%20Reference) (OtherBodyIndex :type Integer) (bFromSweep :type Boolean) (SweepResult :type Hit%20Result%20Structure%20%28by%20ref%29))
  (Variables|Default|SetOverlappedActor OtherActor)
  ;[1 1 1] Check actor implements the NPC Controller BPI
  (Utilities|IsValid (Actor|GetComponentbyClass (Variables|Default|GetOverlappedActor) "/Game/NPCManager/Blueprints/Characters/NPC/Comp_NPC_Controller.Comp_NPC_Controller_C")
    (:Is%20Valid
      (bind _output_get (Variables|Default|SetNPC_Controller (Actor|GetComponentbyClass (Variables|Default|GetOverlappedActor) "/Game/NPCManager/Blueprints/Characters/NPC/Comp_NPC_Controller.Comp_NPC_Controller_C")))
      (if (Utilities|DoesObjectImplementInterface _output_get "/Game/NPCManager/Blueprints/Core/Interfaces/BPI_NPC_Controller.BPI_NPC_Controller_C")
        ;[1 1 1] Send message - Arrived at POI
        (Class|BPINPCController|FnArrivedatPOI(Message) (Variables|Default|GetNPC_Controller) (Variables|Setup|GetParentPOI))))))

(fn ConstructionScript
  ;[1 1 1] Set Entrance visibility
  (Rendering|SetVisibility (Variables|Default|GetEntrance) (Variables|Setup|GetEntranceVisible) false)
  (Development|SetHiddeninGame (Variables|Default|GetEntrance) (Variables|Setup|GetEntranceHidden) false))