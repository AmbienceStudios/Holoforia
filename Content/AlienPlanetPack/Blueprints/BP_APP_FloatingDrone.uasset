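; Floating drone actor that turns its mesh to face the player's camera when the camera comes within a set distance.
; The construction script applies the chosen mesh and stores its original transform values.
; Each tick interpolates rotation toward the current target, then updates that target to the camera or original rotation, turning faster when tracking and slower otherwise.
; A timeline for vertical hovering is present but never triggered, so the drone does not bob.
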(event EventBeginPlay)

(event Collision|EventActorBeginOverlap
  (params (OtherActor :type Actor%20Object%20Reference)))

(event EventTick
  (params (DeltaSeconds :type Float%20%28single-precision%29))
  (bind _mesh (Variables|Default|GetMesh))
  (Utilities|FlowControl|Sequence
    (:then_0
      (Transformation|SetWorldRotation _mesh (Math|Interpolation|RInterpTo (Transformation|GetWorldRotation _mesh) (Variables|Default|GetRotationTarget) (Utilities|Time|GetWorldDeltaSeconds) (select (Variables|Default|GetLookingAtPlayer) 6.0 1.5)) false false) ; Apply Look at Player Rotation
    )
    (:then_1
      (|FindLookatPlayerRotation))))

(fn ConstructionScript
  (bind _mesh (Variables|Default|GetMesh))
  (bind _returnvalue (Transformation|GetWorldRotation _mesh))
  (Components|StaticMesh|SetStaticMesh (Variables|Default|GetMesh) (Variables|Default|GetStaticMesh))
  (Variables|Default|SetOriginalLocation (Transformation|GetWorldLocation _mesh))
  (Variables|Default|SetOriginalRotation _returnvalue)
  (Variables|Default|SetRotationTarget _returnvalue))