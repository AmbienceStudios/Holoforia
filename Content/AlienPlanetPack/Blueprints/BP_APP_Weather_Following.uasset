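; Weather actor that keeps a configurable particle effect centred on the player's camera, such as rain or ground mist that follows the view.
; The construction script assigns the chosen ParticleEffect as the particle system template.
; From BeginPlay, a looping 0.2-second delay, used instead of Tick, moves the particle system to the camera location.
; With GroundEffect enabled, it follows only in X and Y and keeps the actor root's height.
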(event EventBeginPlay
  (bind _returnvalue (Game|GetPlayerCameraManager 0))
  (bind _returnvalue_2 (Camera|GetCameraLocation _returnvalue))
  (bind (_x _y) (Math|Vector|BreakVector _returnvalue_2))
  (Utilities|FlowControl|Delay 0.2 :!label _label)
  (Transformation|SetWorldLocation (Variables|Default|GetParticleSystem) (select (Variables|Default|GetGroundEffect) (Math|Vector|MakeVector _x _y (.Z (Math|Vector|BreakVector (Transformation|GetWorldLocation (Variables|Default|GetDefaultSceneRoot))))) (Camera|GetCameraLocation (Game|GetPlayerCameraManager 0))) false false)
  (goto _label))

(event Collision|EventActorBeginOverlap
  (params (OtherActor :type Actor%20Object%20Reference)))

(event EventTick
  (params (DeltaSeconds :type Float%20%28single-precision%29)))

(fn ConstructionScript
  (Effects|Components|ParticleSystem|SetTemplate (Variables|Default|GetParticleSystem) (Variables|Default|GetParticleEffect)))