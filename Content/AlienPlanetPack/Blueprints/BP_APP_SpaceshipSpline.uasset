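; BP_APP_SpaceshipSpline is an Alien Planet Pack actor that moves a spaceship mesh along a spline path.
; The construction script applies the chosen static mesh and scale, then places it at the starting distance for an editor preview.
; Each Tick adds Speed to Distance without delta-time scaling and sets the mesh's world transform from the spline's location and rotation there.
; Distance never wraps or resets.
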(event EventTick
  (params (DeltaSeconds :type Float%20%28single-precision%29))
  (bind _spline (Variables|Default|GetSpline))
  (bind _output_get (Variables|Default|SetDistance (+ (Variables|Default|GetDistance) (Variables|Default|GetSpeed))))
  (Transformation|SetWorldTransform (Variables|Default|GetMesh) (Math|Transform|MakeTransform (Spline|GetLocationatDistanceAlongSpline _spline _output_get "World") (Spline|GetRotationatDistanceAlongSpline _spline _output_get "World") (Math|Conversions|ToVector(Float) (Variables|Default|GetScale))) false false))

(fn ConstructionScript
  (bind _spline (Variables|Default|GetSpline))
  (bind _distance (Variables|Default|GetDistance))
  (bind _mesh (Variables|Default|GetMesh))
  (Components|StaticMesh|SetStaticMesh _mesh (Variables|Default|GetStaticMesh))
  (Transformation|SetWorldScale3D _mesh (Math|Conversions|ToVector(Float) (Variables|Default|GetScale)))
  (Transformation|SetWorldTransform (Variables|Default|GetMesh) (Math|Transform|MakeTransform (Spline|GetLocationatDistanceAlongSpline _spline _distance "World") (Spline|GetRotationatDistanceAlongSpline _spline _distance "World") (Math|Conversions|ToVector(Float) (Variables|Default|GetScale))) false false))