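; Player-drivable car with throttle, steering, handbrake, horn, timeline-animated doors and switchable first- and third-person cameras.
; Tick feeds engine RPM to the sound, and speed and RPM to the HUD widget and dashboard materials.
; Dynamic material instances drive headlight, panel, brake, reverse and turn-signal lighting.
; Turn signals blink with sound through timers that re-trigger each other, and auto-cancel based on steering angle.
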(event EventTick
  (params (DeltaSeconds :type Float%20%28single-precision%29))
  ;[1 1 1] Events
  (CallFunction|SteeringAngleUpdate)
  (CallFunction|TurnSignalAutoUpdate)
  (CallFunction|BrakeLightsUpdate)
  (CallFunction|UpdateSpeed/RPM)
  (CallFunction|ReverseLight)
  (Audio|Parameter|SetFloatParameter (Variables|Default|GetEngineSound) "RPM" (Class|WheeledVehicleMovementComponent|GetEngineRotationSpeed (Variables|Default|GetVehicleMovement)) :!class /Script/Engine.AudioComponent))

(event EventBeginPlay
  ;[1 1 1] Events
  (bind _returnvalue (UserInterface|CreateWidget "/Game/CarZ_01/Blueprints/UI/WGB_Speedometer.WGB_Speedometer_C"))
  (bind _output_get (Variables|Default|SetSpeedometer%20UI _returnvalue))
  (UserInterface|Viewport|AddtoViewport _output_get 0))

(event Input|ActionEvents|InputActionSwitchCamera
  (params (Key :type Key%20Structure))
  (bind _speedometer_ui (Variables|Default|GetSpeedometer%20UI))
  ;[1 1 1] Switch Camera
  (:Pressed
    (Utilities|FlowControl|FlipFlop
      (:A
        (Components|Activation|Deactivate (Variables|Default|GetThirdPersonCamera))
        (Components|Activation|SetActive (Variables|Default|GetFirstPersonCamera) true false)
        (Transformation|SetRelativeRotation (Variables|Default|GetFirstPersonCamera) "-10.000000, 0, 0" false false)
        (Widget|SetVisibility _speedometer_ui "Hidden"))
      (:B
        (Components|Activation|Deactivate (Variables|Default|GetFirstPersonCamera))
        (Components|Activation|SetActive (Variables|Default|GetThirdPersonCamera) true false)
        (Transformation|SetRelativeRotation (Variables|Default|GetSpringArm) "-10.000000, 0, 0" false false)
        (Widget|SetVisibility _speedometer_ui "Visible")))))

(event Input|ActionEvents|InputActionLeftDoorTrigger
  (params (Key :type Key%20Structure))
  ;[1 1 1] Door Funtionality
  (:Pressed
    (Utilities|FlowControl|FlipFlop
      (:A
        (bind _door_angle (Timeline|Left%20Door Play)
          (:Update
            (Variables|Default|SetLeft%20Door%20Angle _door_angle))))
      (:B
        (Timeline|Left%20Door Reverse)))))

(event Input|ActionEvents|InputActionRightDoorTrigger
  (params (Key :type Key%20Structure))
  ;[1 1 1] Door Funtionality
  (:Pressed
    (Utilities|FlowControl|FlipFlop
      (:A
        (bind _door_angle (Timeline|Right%20Door Play)
          (:Update
            (Variables|Default|SetRight%20Door%20Angle _door_angle))))
      (:B
        (Timeline|Right%20Door Reverse)))))

(event Input|ActionEvents|InputActionHandBrake
  (params (Key :type Key%20Structure))
  (bind _vehiclemovement (Variables|Default|GetVehicleMovement))
  ;[1 1 1] HandBrake
  (:Pressed
    (Class|WheeledVehicleMovementComponent|SetHandbrakeInput _vehiclemovement true))
  (:Released
    (Class|WheeledVehicleMovementComponent|SetHandbrakeInput _vehiclemovement false)))

(event Input|ActionEvents|InputActionHandBrake
  (params (Key :type Key%20Structure))
  ;[1 1 1] Lights
  (:Pressed
    (Variables|Default|SetLights%20on true))
  (:Released
    (Variables|Default|SetLights%20on false)))

(event Input|ActionEvents|InputActionPanelLights
  (params (Key :type Key%20Structure))
  (bind _tachometer (Variables|Default|GetTachometer))
  (bind _panel_lights (Variables|Default|GetPanel%20Lights))
  (bind _speedometer (Variables|Default|GetSpeedometer))
  ;[1 1 1] Lights
  (:Pressed
    (Utilities|FlowControl|FlipFlop
      (:A
        (Rendering|Material|SetScalarParameterValue _speedometer "Panel Emission" 0.0 :!class /Script/Engine.MaterialInstanceDynamic)
        (Rendering|Material|SetScalarParameterValue _tachometer "Panel Emission" 0.0 :!class /Script/Engine.MaterialInstanceDynamic)
        (Rendering|Material|SetScalarParameterValue _panel_lights "Panel Emission" 0.0 :!class /Script/Engine.MaterialInstanceDynamic))
      (:B
        (Rendering|Material|SetScalarParameterValue _speedometer "Panel Emission" 1.0 :!class /Script/Engine.MaterialInstanceDynamic)
        (Rendering|Material|SetScalarParameterValue _tachometer "Panel Emission" 1.0 :!class /Script/Engine.MaterialInstanceDynamic)
        (Rendering|Material|SetScalarParameterValue _panel_lights "Panel Emission" 1.0 :!class /Script/Engine.MaterialInstanceDynamic)))))

(event Input|ActionEvents|InputActionHeadLamps
  (params (Key :type Key%20Structure))
  (bind _car_lights (Variables|Default|GetCar%20Lights))
  (bind _headlamp (Variables|Default|GetHeadLamp))
  (bind _headlamps (Variables|Default|GetHeadlamps))
  ;[1 1 1] Lights
  (:Pressed
    (Utilities|FlowControl|FlipFlop
      (:A
        (Rendering|Material|SetScalarParameterValue _car_lights "Headlight" 5.0 :!class /Script/Engine.MaterialInstanceDynamic)
        (Rendering|SetVisibility _headlamp true false)
        (Rendering|SetVisibility _headlamps true false))
      (:B
        (Rendering|Material|SetScalarParameterValue _car_lights "Headlight" 0.2 :!class /Script/Engine.MaterialInstanceDynamic)
        (Rendering|SetVisibility _headlamp false false)
        (Rendering|SetVisibility _headlamps false false)))))

(event Input|ActionEvents|InputActionTurnLeftSIgnal
  (params (Key :type Key%20Structure))
  ;[1 1 1] Turn Signal Inputs
  (:Pressed
    (if (Variables|Default|GetLeft%20Turn%20Activated)
      (Variables|Default|SetLeft%20Turn%20Activated false)
      (CallFunction|TurnOffLeftSignal)
      (else
        (Variables|Default|SetLeft%20Turn%20Activated true)
        (CallFunction|TurnonLeftSignal)))))

(event Input|ActionEvents|InputActionTurnRightSignal
  (params (Key :type Key%20Structure))
  ;[1 1 1] Turn Signal Inputs
  (:Pressed
    (if (Variables|Default|GetRight%20Turn%20Activated)
      (Variables|Default|SetRight%20Turn%20Activated false)
      (CallFunction|TurnOffRightSignal)
      (else
        (Variables|Default|SetRight%20Turn%20Activated true)
        (CallFunction|TurnonRightSignal)))))

(event Input|ActionEvents|InputActionHorn
  (params (Key :type Key%20Structure))
  (bind _horn (Variables|Default|GetHorn))
  ;[1 1 1] Car Horn
  (:Pressed
    (Components|Activation|SetActive _horn true false))
  (:Released
    (Components|Activation|SetActive _horn false false)))

(event Input|AxisEvents|InputAxisLookUp
  (params (AxisValue :type Float%20%28single-precision%29))
  ;[1 1 1] Camera LookAround
  (if (Components|Activation|IsActive (Variables|Default|GetFirstPersonCamera))
    (Transformation|AddRelativeRotation (Variables|Default|GetFirstPersonCamera) (Math|Rotator|MakeRotator 0.0 AxisValue 0.0) false false)
    (else
      (Transformation|AddRelativeRotation (Variables|Default|GetSpringArm) (Math|Rotator|MakeRotator 0.0 AxisValue 0.0) false false))))

(event Input|AxisEvents|InputAxisLookRight
  (params (AxisValue :type Float%20%28single-precision%29))
  ;[1 1 1] Camera LookAround
  (if (Components|Activation|IsActive (Variables|Default|GetFirstPersonCamera))
    (Transformation|AddRelativeRotation (Variables|Default|GetFirstPersonCamera) (Math|Rotator|MakeRotator 0.0 0.0 AxisValue) false false)
    (else
      (Transformation|AddRelativeRotation (Variables|Default|GetSpringArm) (Math|Rotator|MakeRotator 0.0 0.0 AxisValue) false false))))

(event Input|AxisEvents|InputAxisMoveForward
  (params (AxisValue :type Float%20%28single-precision%29))
  ;[1 1 1] Steering And Throtle
  (Class|WheeledVehicleMovementComponent|SetThrottleInput (Variables|Default|GetVehicleMovement) AxisValue))

(event Input|AxisEvents|InputAxisMoveRight
  (params (AxisValue :type Float%20%28single-precision%29))
  ;[1 1 1] Steering And Throtle
  (Class|WheeledVehicleMovementComponent|SetSteeringInput (Variables|Default|GetVehicleMovement) AxisValue))

(fn ConstructionScript
  (bind _returnvalue (Rendering|Material|CreateDynamicMaterialInstance (Variables|Character|GetMesh) 1 0 "None" :!class /Script/Engine.PrimitiveComponent))
  (Variables|Default|SetCar%20Lights _returnvalue)
  (bind _returnvalue_2 (Rendering|Material|CreateDynamicMaterialInstance (Variables|Character|GetMesh) 5 0 "None" :!class /Script/Engine.PrimitiveComponent))
  (Variables|Default|SetSpeedometer _returnvalue_2)
  (bind _returnvalue_3 (Rendering|Material|CreateDynamicMaterialInstance (Variables|Character|GetMesh) 6 0 "None" :!class /Script/Engine.PrimitiveComponent))
  (Variables|Default|SetTachometer _returnvalue_3)
  (bind _returnvalue_4 (Rendering|Material|CreateDynamicMaterialInstance (Variables|Character|GetMesh) 3 0 "None" :!class /Script/Engine.PrimitiveComponent))
  (Variables|Default|SetPanel%20Lights _returnvalue_4)
  (Rendering|Material|CreateDynamicMaterialInstance (Variables|Character|GetMesh) 1 0 "None" :!class /Script/Engine.PrimitiveComponent))

(fn SteeringAngleUpdate
  (bind _vehiclemovement (Variables|Default|GetVehicleMovement))
  (bind _wheels (Variables|/Script/PhysXVehicles.WheeledVehicleMovementComponent|GetWheels _vehiclemovement))
  (bind _output (Utilities|Array|Get(acopy) _wheels))
  (bind _output_2 (Utilities|Array|Get(acopy) _wheels 1))
  (bind _returnvalue (Class|VehicleWheel|GetSteerAngle _output_2))
  (bind _returnvalue_2 (Class|VehicleWheel|GetSteerAngle _output))
  (Variables|Default|SetSteering%20Angle (Math|Float|SelectFloat _returnvalue_2 _returnvalue (> (Math|Float|Absolute(Float) _returnvalue_2) (Math|Float|Absolute(Float) _returnvalue)))))

(fn BrakeLightsUpdate
  (bind _car_lights (Variables|Default|GetCar%20Lights))
  (if (< (* (Class|WheeledVehicleMovementComponent|GetForwardSpeed (Variables|Default|GetVehicleMovement)) (Input|AxisValues|GetMoveForward)) -5.0)
    (Rendering|Material|SetScalarParameterValue _car_lights "BrakeLights" 1e+01 :!class /Script/Engine.MaterialInstanceDynamic)
    (else
      (Rendering|Material|SetScalarParameterValue _car_lights "BrakeLights" (Math|Float|SelectFloat 1e+01 0.1 (Variables|Default|GetLights%20on)) :!class /Script/Engine.MaterialInstanceDynamic))))

(fn UpdateSpeed/RPM
  (bind _vehiclemovement (Variables|Default|GetVehicleMovement))
  (bind _returnvalue (Class|WheeledVehicleMovementComponent|GetForwardSpeed _vehiclemovement))
  (bind _returnvalue_2 (Class|WheeledVehicleMovementComponent|GetEngineRotationSpeed _vehiclemovement))
  (bind _returnvalue_3 (/ _returnvalue_2 8e+03))
  (bind _returnvalue_4 (* _returnvalue 0.036))
  (bind _returnvalue_5 (/ _returnvalue_4 2.4e+02))
  (bind _returnvalue_6 (Math|Float|Absolute(Float) _returnvalue_5))
  (Default|UpdateHUD (Variables|Default|GetSpeedometer%20UI) _returnvalue_6 _returnvalue_3)
  (Rendering|Material|SetScalarParameterValueonMaterials (Variables|Character|GetMesh) "Value" _returnvalue_3)
  (Rendering|Material|SetScalarParameterValueonMaterials (Variables|Character|GetMesh) "SpeedValue" _returnvalue_6))

(fn TurnonLeftSignal
  (bind _turn_signal (Variables|Default|GetTurn%20Signal))
  (if (Variables|Default|GetLeft%20Turn%20Activated)
    (Rendering|Material|SetScalarParameterValue (Variables|Default|GetCar%20Lights) "Left Trafig" 1e+01 :!class /Script/Engine.MaterialInstanceDynamic)
    (Audio|Components|Audio|SetSound _turn_signal "/Game/CarZ_01/Sounds/Signal_Turn_on.Signal_Turn_on")
    (Audio|Components|Audio|Play _turn_signal 0.0)
    (Utilities|Time|SetTimerbyFunctionName 0 "Turn Off Left Signal" 0.3)))

(fn TurnonRightSignal
  (bind _turn_signal (Variables|Default|GetTurn%20Signal))
  (if (Variables|Default|GetRight%20Turn%20Activated)
    (Rendering|Material|SetScalarParameterValue (Variables|Default|GetCar%20Lights) "Right Trafig" 1e+01 :!class /Script/Engine.MaterialInstanceDynamic)
    (Audio|Components|Audio|SetSound _turn_signal "/Game/CarZ_01/Sounds/Signal_Turn_on.Signal_Turn_on")
    (Audio|Components|Audio|Play _turn_signal 0.0)
    (Utilities|Time|SetTimerbyFunctionName 0 "Turn Off Right Signal" 0.3)))

(fn TurnOffRightSignal
  (bind _turn_signal (Variables|Default|GetTurn%20Signal))
  (bind _returnvalue (Rendering|Material|GetScalarParameterValue (Variables|Default|GetCar%20Lights) "Right Trafig" :!class /Script/Engine.MaterialInstanceDynamic))
  (if (> _returnvalue 0.0)
    (Rendering|Material|SetScalarParameterValue (Variables|Default|GetCar%20Lights) "Right Trafig" 0.2 :!class /Script/Engine.MaterialInstanceDynamic)
    (Audio|Components|Audio|SetSound _turn_signal "/Game/CarZ_01/Sounds/Signal_Turn_off.Signal_Turn_off")
    (Audio|Components|Audio|Play _turn_signal 0.0)
    (if (Variables|Default|GetRight%20Turn%20Activated)
      (Utilities|Time|SetTimerbyFunctionName 0 "Turn on Right Signal" 0.5))))

(fn TurnOffLeftSignal
  (bind _turn_signal (Variables|Default|GetTurn%20Signal))
  (bind _returnvalue (Rendering|Material|GetScalarParameterValue (Variables|Default|GetCar%20Lights) "Left Trafig" :!class /Script/Engine.MaterialInstanceDynamic))
  (if (> _returnvalue 0.0)
    (Rendering|Material|SetScalarParameterValue (Variables|Default|GetCar%20Lights) "Left Trafig" 0.2 :!class /Script/Engine.MaterialInstanceDynamic)
    (Audio|Components|Audio|SetSound _turn_signal "/Game/CarZ_01/Sounds/Signal_Turn_off.Signal_Turn_off")
    (Audio|Components|Audio|Play _turn_signal 0.0)
    (if (Variables|Default|GetLeft%20Turn%20Activated)
      (Utilities|Time|SetTimerbyFunctionName 0 "Turn on Left Signal" 0.5))))

(fn TurnSignalAutoUpdate
  (bind _steering_angle (Variables|Default|GetSteering%20Angle))
  (Utilities|FlowControl|Sequence
    (:then_0
      (if (Variables|Default|GetLeft%20Turn%20Activated)
        (if (and (Variables|Default|GetLeft%20Turn%20can%20be%20Deactivated) (> _steering_angle -2e+01))
          (Variables|Default|SetLeft%20Turn%20Activated false)
          (Variables|Default|SetLeft%20Turn%20can%20be%20Deactivated false)
          (CallFunction|TurnOffLeftSignal)
          (elif (< _steering_angle -2e+01)
            (Variables|Default|SetLeft%20Turn%20can%20be%20Deactivated true)))))
    (:then_1
      (if (Variables|Default|GetRight%20Turn%20Activated)
        (if (and (Variables|Default|GetRight%20Turn%20can%20be%20Deactivated) (> (Variables|Default|GetSteering%20Angle) 2e+01))
          (Variables|Default|SetRight%20Turn%20Activated false)
          (Variables|Default|SetRight%20Turn%20can%20be%20Deactivated false)
          (CallFunction|TurnOffRightSignal)
          (elif (< (Variables|Default|GetSteering%20Angle) 2e+01)
            (Variables|Default|SetRight%20Turn%20can%20be%20Deactivated true)))))))

(fn ReverseLight
  (bind _car_lights (Variables|Default|GetCar%20Lights))
  (if (< (Class|WheeledVehicleMovementComponent|GetForwardSpeed (Variables|Default|GetVehicleMovement)) -2.0)
    (Rendering|Material|SetScalarParameterValue _car_lights "Reverse Light" 5.0 :!class /Script/Engine.MaterialInstanceDynamic)
    (else
      (Rendering|Material|SetScalarParameterValue _car_lights "Reverse Light" 0.2 :!class /Script/Engine.MaterialInstanceDynamic))))