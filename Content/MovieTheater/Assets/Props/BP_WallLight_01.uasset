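; BP_WallLight_01 is a wall light prop for the movie theater, with two spotlights configured in the Construction Script.
; When Lit is set, both spotlights receive the shared intensity, indirect intensity, cone angles, radius and color temperature variables.
; Otherwise their attenuation radius is set to zero, rather than changing intensity or visibility.
; The event graph holds no runtime logic.
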(event EventBeginPlay)

(event Collision|EventActorBeginOverlap
  (params (OtherActor :type Actor%20Object%20Reference)))

(event EventTick
  (params (DeltaSeconds :type Float%20%28single-precision%29)))

(fn ConstructionScript
  (bind _spotlight1 (Variables|Default|GetSpotLight1))
  (bind _spotlight2 (Variables|Default|GetSpotLight2))
  (bind _array (Utilities|Array|MakeArray _spotlight1 _spotlight2 0 0))
  (if (Variables|Default|GetLit)
    (for _array_element (Utilities|Array|MakeArray _spotlight2 _spotlight1)
      (Class|LightComponent|SetIndirectLightingIntensity _array_element (Variables|Default|GetIndirect%20Intensity))
      (Rendering|Lighting|SetInnerConeAngle _array_element (Variables|Range|GetInner%20Cone%20Range))
      (Rendering|Lighting|SetOuterConeAngle _array_element (Variables|Range|GetOuter%20Cone%20Range))
      (Rendering|Lighting|SetAttenuationRadius _array_element (Variables|Range|GetRadius))
      (Rendering|Components|Light|SetIntensity _array_element (Variables|Default|GetIntensity))
      (Class|LightComponent|SetTemperature _array (Variables|Default|GetTemperature)))
    (else
      (for _array_element_2 _array
        (Rendering|Lighting|SetAttenuationRadius _array_element_2 0.0)
        (Rendering|Lighting|SetAttenuationRadius _array_element_2 0.0)))))