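; BP_FlameMachine01 is a dance club stage flame machine that fires bursts of flame at random intervals.
; Tick feeds a Delay with a random time between PeriodMin and PeriodMax, so the burst repeats without an explicit timer or loop.
; Each burst activates the particle system and audio, then restarts a timeline whose Brightness curve, scaled by LightBrightness, drives the point light's intensity.
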(event EventBeginPlay)

(event Collision|EventActorBeginOverlap
  (params (OtherActor :type Actor%20Object%20Reference)))

(event EventTick
  (params (DeltaSeconds :type Float%20%28single-precision%29))
  ;[1 1 1] Flame machine emmite flames randomly, throw time period controlled by the "Period Min/Max" values
  (Utilities|FlowControl|Delay (Math|Random|RandomFloatinRange (Variables|Default|GetPeriodMin) (Variables|Default|GetPeriodMax)))
  (Components|Activation|Activate (Variables|Default|GetParticleSystem) false)
  (Components|Activation|Activate (Variables|Default|GetAudio) false)
  (bind _brightness (Timeline|Timeline_0 PlayFromStart)
    (:Update
      (Rendering|Components|Light|SetIntensity (Variables|Default|GetPointLight) (* _brightness (Variables|Default|GetLightBrightness))))))

(fn ConstructionScript)