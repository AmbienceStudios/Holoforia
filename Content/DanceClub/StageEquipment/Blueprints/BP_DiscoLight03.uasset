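; BP_DiscoLight03 is a dance club stage light prop with a spinning base and two rotating disco balls.
; Every Tick it yaws the base mesh at BaseSpeed and rolls the two ball meshes in opposite directions at BallsSpeed.
; Rotations are local and scaled by delta seconds, so the motion is frame-rate independent; the construction script is empty.
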(event EventBeginPlay)

(event Collision|EventActorBeginOverlap
  (params (OtherActor :type Actor%20Object%20Reference)))

(event EventTick
  (params (DeltaSeconds :type Float%20%28single-precision%29))
  (bind _ballsspeed (Variables|Default|GetBallsSpeed))
  (bind _returnvalue (* _ballsspeed DeltaSeconds))
  (bind _returnvalue_2 (Math|Rotator|MakeRotator _returnvalue 0.0 0.0))
  ;[1 1 1] Balls base and balls rotation speed controller
  (Transformation|AddLocalRotation (Variables|Default|GetStaticMeshComponent02) (Math|Rotator|MakeRotator 0.0 0.0 (* (Variables|Default|GetBaseSpeed) DeltaSeconds)) false false)
  (Transformation|AddLocalRotation (Variables|Default|GetStaticMeshComponent0) _returnvalue_2 false false)
  (Transformation|AddLocalRotation (Variables|Default|GetStaticMeshComponent01) (Class|KismetMathLibrary|NegateRotator _returnvalue_2) false false))

(fn ConstructionScript)