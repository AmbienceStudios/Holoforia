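; BP_HeaderData is an Xsolla data Blueprint holding a display name, an avatar URL and the avatar brush, apparently for a header.
; The RefreshIcon event stores the supplied icon as the avatar and flags it as ready.
; Getters expose the name, URL, ready state and avatar, with GetAvatar returning a default small sized brush whenever the URL is empty.
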(event EventRefreshIcon
  (params (Icon :type Slate%20Brush%20Structure))
  (Variables|Default|SetAvatar Icon)
  (Variables|Default|SetIsAvatarReady true))

(fn GetAvatar
  (return (select (> (Utilities|String|Len (Variables|Default|GetAvatarUrl)) 0) (Variables|Default|GetAvatar) (Utilities|Struct|MakeSlateBrush "(X=27.000000,Y=27.000000)" "(Left=0.000000,Top=0.000000,Right=0.000000,Bottom=0.000000)" "(SpecifiedColor=(R=1.000000,G=1.000000,B=1.000000,A=1.000000),ColorUseRule=UseColor_Specified)" "/Game/MRPGInventorySystem/XSolla/Common/Assets/Avatars/T_AvatarPlaceholder.T_AvatarPlaceholder" "Image" "NoTile" "NoMirror"))))

(fn GetDisplayName
  (return (Variables|Default|GetDisplayName)))

(fn GetImageUrl
  (return (Variables|Default|GetAvatarUrl)))

(fn IsIconSet
  (return (Variables|Default|GetIsAvatarReady)))