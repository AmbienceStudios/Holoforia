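; BP_VCBalanceItemData is a data wrapper for one virtual currency balance entry in the Xsolla inventory.
; Getter functions expose the amount, description, image URL, name and SKU from its ItemData struct.
; The icon is stored separately: the RefreshIcon event sets it and raises IsIconReady, which IsIconSet reports alongside GetIcon.
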(event EventRefreshIcon
  (params (Icon :type Slate%20Brush%20Structure))
  (Variables|Default|SetIcon Icon)
  (Variables|Default|SetIsIconReady true))

(fn GetAmount
  (return (.amount (Utilities|Struct|BreakVirtualCurrencyBalance (Variables|Default|GetItemData)))))

(fn GetDescription
  (return (.description (Utilities|Struct|BreakVirtualCurrencyBalance (Variables|Default|GetItemData)))))

(fn GetIcon
  (return (Variables|Default|GetIcon)))

(fn GetImageUrl
  (return (.image_url (Utilities|Struct|BreakVirtualCurrencyBalance (Variables|Default|GetItemData)))))

(fn GetName
  (return (.name (Utilities|Struct|BreakVirtualCurrencyBalance (Variables|Default|GetItemData)))))

(fn GetSku
  (return (.sku (Utilities|Struct|BreakVirtualCurrencyBalance (Variables|Default|GetItemData)))))

(fn IsIconSet
  (return (Variables|Default|GetIsIconReady)))