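; BP_VCPrice is a data object for a virtual currency price in the XSolla store integration of the inventory system.
; It exposes getters for SKU, amount, amount without discount, image URL and icon.
; A RefreshIcon event stores a supplied icon and sets a ready flag, which IsIconSet reports.
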(event EventRefreshIcon
  (params (Icon :type Slate%20Brush%20Structure))
  (Variables|Default|SetIcon Icon)
  (Variables|Default|SetIsIconReady true))

(fn GetAmount
  (return (Variables|Default|GetAmount)))

(fn GetAmountWithoutDiscount
  (return (Variables|Default|GetAmountWithoutDiscount)))

(fn GetIcon
  (return (Variables|Default|GetIcon)))

(fn GetImageUrl
  (return (Variables|Default|GetImageUrl)))

(fn GetSku
  (return (Variables|Default|GetSku)))

(fn IsIconSet
  (return (Variables|Default|GetIsIconReady)))