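; BP_BundleItemData is a data object that wraps an Xsolla store bundle and exposes its SKU, name, image URL, content and prices.
; Getters read from ItemData, formatting the price and total content price with their currencies.
; GetPriceVC lazily creates and caches a BP_VCPrice from the first virtual price, if one exists.
; RefreshIcon stores a supplied icon and flags it ready for IsIconSet.
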(event EventRefreshIcon
  (params (Icon :type Slate%20Brush%20Structure))
  (Variables|Default|SetIcon Icon)
  (Variables|Default|SetIsIconReady true))

(fn GetContent
  (return (Utilities|Struct|BreakStoreBundle (Variables|Default|GetItemData))))

(fn GetFullPrice
  (bind _itemdata (Variables|Default|GetItemData))
  (bind _total_content_price (Utilities|Struct|BreakStoreBundle _itemdata))
  (bind (_amount _amount_without_discount _currency) (Utilities|Struct|BreakXsollaPrice _total_content_price))
  (return (Class|XsollaStoreLibrary|FormatPrice (Math|Conversions|ToFloat(Integer) _amount) _currency)))

(fn GetIcon
  (return (Variables|Default|GetIcon)))

(fn GetImageUrl
  (return (Utilities|Struct|BreakStoreBundle (Variables|Default|GetItemData))))

(fn GetName
  (return (Utilities|Struct|BreakStoreBundle (Variables|Default|GetItemData))))

(fn GetPrice
  (bind _itemdata (Variables|Default|GetItemData))
  (bind _price (Utilities|Struct|BreakStoreBundle _itemdata))
  (bind (_amount _amount_without_discount _currency) (Utilities|Struct|BreakXsollaPrice _price))
  (return (Class|XsollaStoreLibrary|FormatPrice (Math|Conversions|ToFloat(Integer) _amount) _currency)))

(fn GetPriceVC
  (bind _itemdata (Variables|Default|GetItemData))
  (bind _virtual_prices (Utilities|Struct|BreakStoreBundle _itemdata))
  (bind _output (Utilities|Array|Get(acopy) _virtual_prices))
  (bind (_sku _is_default _amount _amount_without_discount _image_url) (Utilities|Struct|BreakXsollaVirtualCurrencyPrice _output))
  (Utilities|IsValid (Variables|Default|GetVCPrice)
    (:Is%20Valid
      (return (Variables|Default|GetVCPrice)))
    (:Is%20Not%20Valid
      (if (> (Utilities|Array|Length _virtual_prices) 0)
        (bind _returnvalue (Game|ConstructObjectfromClass "/Game/MRPGInventorySystem/XSolla/Store/Data/BP_VCPrice.BP_VCPrice_C" self _sku _amount _amount_without_discount _image_url))
        (bind _output_get (Variables|Default|SetVCPrice _returnvalue))
        (return _output_get)))))

(fn GetSku
  (return (Utilities|Struct|BreakStoreBundle (Variables|Default|GetItemData))))

(fn IsIconSet
  (return (Variables|Default|GetIsIconReady)))