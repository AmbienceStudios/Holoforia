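; Data object for one social network entry in the Xsolla Login integration.
; It stores the provider, its icon, whether it is linked, and a parent reference.
; Four getter functions expose these values, with no other logic.
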(fn GetParent
  (return (Variables|Default|GetParent)))

(fn GetProvider
  (return (Variables|Default|GetProvider)))

(fn GetProviderIcon
  (return (Variables|Default|GetIcon)))

(fn GetStatus
  (return (Variables|Default|GetIsLinked)))