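; Blueprint function library of shared lookup helpers for the RPG inventory system.
; Item data comes from the DT_InventoryItems table by row name, while equipment type is looked up by item ID in EquipmentComponent class defaults.
; HUD and inventory manager getters read from player 0's InventoryPlayerController after a validity check.
; GetOwningCharacter resolves a component's character by casting its owner to that controller class.
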(fn GetItemData
  (params (ItemID :type Name))
  (bind _returnvalue (Utilities|GetDataTableRow "/Game/MRPGInventorySystem/Data/DT_InventoryItems.DT_InventoryItems" ItemID)
    (:then
      (return _returnvalue))
    (:RowNotFound
      (return ""))))

(fn GetEquipmentType
  (params (ItemID :type Integer))
  (return (Utilities|Array|Get(acopy) (Utilities|GetClassDefaults "/Game/MRPGInventorySystem/Blueprints/Components/EquipmentComponent.EquipmentComponent_C") ItemID)))

(fn GetInventoryPlayerController
  (return (.AsInventory%20Player%20Controller (Utilities|Casting|CastToInventoryPlayerController (Game|GetPlayerController 0)))))

(fn GetInventoryHUD
  (bind _returnvalue (Game|GetPlayerController 0))
  (bind _asinventory_player_controller (Utilities|Casting|CastToInventoryPlayerController _returnvalue))
  (Utilities|IsValid _asinventory_player_controller
    (:Is%20Valid
      (return (Variables|/Game/MRPGInventorySystem/Blueprints/InventoryPlayerController.InventoryPlayerController_C|GetHud _asinventory_player_controller)))
    (:Is%20Not%20Valid
      (return 0))))

(fn GetInventoryManager
  (bind _returnvalue (Game|GetPlayerController 0))
  (bind _asinventory_player_controller (Utilities|Casting|CastToInventoryPlayerController _returnvalue))
  (Utilities|IsValid _asinventory_player_controller
    (:Is%20Valid
      (return (Variables|/Game/MRPGInventorySystem/Blueprints/InventoryPlayerController.InventoryPlayerController_C|GetInventoryManager _asinventory_player_controller)))
    (:Is%20Not%20Valid
      (return 0))))

(fn GetOwningCharacter
  (params (Component :type Actor%20Component%20Object%20Reference))
  (return (Default|GetInventoryCharacter (.AsInventory%20Player%20Controller (Utilities|Casting|CastToInventoryPlayerController (Components|GetOwner Component))))))