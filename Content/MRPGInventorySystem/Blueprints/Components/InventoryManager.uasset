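; Player-controller component that handles inventory transactions between inventory, equipment, storage and store containers, plus item pickup, drops and gold.
; Server events run the move, stack, swap, equip-check and purchase logic, then send slot and gold changes to every manager watching that container.
; Client events apply those changes to the HUD widgets.
; While a container or store is open, server tick closes it once the player moves away.
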(event Custom|Server_DropItem
  (params (IndexFrom :type Integer) (ContainerFrom :type Items%20Container%20Component%20Object%20Reference))
  ;[1 0.5992 0.4169 0.4 30] Server
  (Server|DropItem IndexFrom ContainerFrom))

(event Custom|InitializeWorldStore
  (params (ContainerItem :type Array%20of%20Container%20Item%20Structures))
  ;[0.04772 0.6094 0.2873 0.4 30] Client
  (Default|InitializeSlots (Variables|/Game/MRPGInventorySystem/UMG/WBP_InventoryHUD.WBP_InventoryHUD_C|GetWorldStore (Utilities|GetMainHud)) ContainerItem))

(event Custom|TrackPlayerOpenedContainer
  (params (IsOpen :type Boolean) (IsStore :type Boolean))
  ;[1 0.5992 0.4169 0.4] Server - track player and close container when player moves
  (Variables|Default|SetObservePlayerPosition (Transformation|GetActorLocation (Pawn|GetControlledPawn (.AsPlayer%20Controller (Utilities|Casting|CastToPlayerController (Components|GetOwner))))))
  (Variables|Default|SetIsStore IsStore)
  (Components|Tick|SetComponentTickEnabled IsOpen))

(event Custom|Server_SetSlot
  (params (ContainerClass :type Items%20Container%20Component%20Object%20Reference) (Index :type Integer) (Item :type Container%20Item%20Structure))
  ;[1 0.5992 0.4169 0.4 30] Server
  (bind _managers (Server|GetWatchingManagers ContainerClass))
  (for _array_element _managers
    (CallFunction|ClientSetSlot _array_element (Utilities|GetClass ContainerClass) Index Item)))

(event Custom|Client_RemoveSlot
  (params (ContainerClass :type Items%20Container%20Component%20Class%20Reference) (Index :type Integer))
  ;[0.04772 0.6094 0.2873 0.4 30] Client
  (Default|RemoveSlot (Default|GetContainerWidget (Utilities|GetMainHud) ContainerClass) Index))

(event Custom|InitializeContainers
  (bind _hud (Utilities|GetMainHud))
  (bind _inventory_character (Utilities|GetInventoryCharacter))
  (bind _playerinventory (Variables|/Game/MRPGInventorySystem/UMG/WBP_InventoryHUD.WBP_InventoryHUD_C|GetPlayerInventory _hud))
  (bind _inventorycomponent (Variables|/Game/MRPGInventorySystem/Blueprints/Actors/BP_InventoryCharacter.BP_InventoryCharacter_C|GetInventoryComponent _inventory_character))
  ;[0.04772 0.6094 0.2873 0.4 30] Client
  (Default|InitializeSlots _playerinventory (Variables|/Game/MRPGInventorySystem/Blueprints/Components/ItemsContainerComponent.ItemsContainerComponent_C|GetContainerItems _inventorycomponent))
  (Default|UpdateGold _playerinventory (Variables|/Game/MRPGInventorySystem/Blueprints/Components/ItemsContainerComponent.ItemsContainerComponent_C|GetGoldAmount _inventorycomponent))
  (Default|UpdateSlots (Variables|/Game/MRPGInventorySystem/UMG/WBP_InventoryHUD.WBP_InventoryHUD_C|GetEquipement _hud) (Variables|/Game/MRPGInventorySystem/Blueprints/Components/ItemsContainerComponent.ItemsContainerComponent_C|GetContainerItems (Variables|/Game/MRPGInventorySystem/Blueprints/Actors/BP_InventoryCharacter.BP_InventoryCharacter_C|GetEquipmentComponent _inventory_character))))

(event Custom|Server_MoveToContainer
  (params (IndexFrom :type Integer) (ContainerFrom :type Items%20Container%20Component%20Object%20Reference) (ContainerTo :type Items%20Container%20Component%20Object%20Reference))
  ;[1 0.5992 0.4169 0.4 30] Server
  (Server|MovetoContainer IndexFrom ContainerFrom ContainerTo))

(event Custom|Client_SetSlot
  (params (ContainerClass :type Items%20Container%20Component%20Class%20Reference) (Index :type Integer) (Item :type Container%20Item%20Structure))
  ;[0.04772 0.6094 0.2873 0.4 30] Client
  (Default|SetSlot (Default|GetContainerWidget (Utilities|GetMainHud) ContainerClass) Index Item))

(event Custom|Server_PickGold
  (params (GoldAmount :type Integer))
  ;[1 0.5992 0.4169 0.4 30] Server
  (Server|PickupGold GoldAmount))

(event Custom|Server_UpdateGold
  (params (ContainerClass :type Items%20Container%20Component%20Object%20Reference))
  ;[1 0.5992 0.4169 0.4 30] Server
  (bind _managers (Server|GetWatchingManagers ContainerClass))
  (for _array_element _managers
    (CallFunction|ClientUpdateGold _array_element (Utilities|GetClass ContainerClass) (Variables|/Game/MRPGInventorySystem/Blueprints/Components/ItemsContainerComponent.ItemsContainerComponent_C|GetGoldAmount ContainerClass))))

(event Custom|Server_AddSlot
  (params (ContainerClass :type Items%20Container%20Component%20Object%20Reference) (Item :type Container%20Item%20Structure))
  ;[1 0.5992 0.4169 0.4 30] Server
  (bind _managers (Server|GetWatchingManagers ContainerClass))
  (for _array_element _managers
    (CallFunction|ClientAddSlot _array_element (Utilities|GetClass ContainerClass) Item)))

(event Custom|Client_UpdateGold
  (params (ContainerClass :type Items%20Container%20Component%20Class%20Reference) (GoldAmount :type Integer))
  ;[0.04772 0.6094 0.2873 0.4 30] Client
  (Default|UpdateGold (Default|GetContainerWidget (Utilities|GetMainHud) ContainerClass) GoldAmount))

(event Custom|Server_MoveToSlot
  (params (IndexFrom :type Integer) (IndexTo :type Integer) (ContainerFrom :type Items%20Container%20Component%20Object%20Reference) (ContainerTo :type Items%20Container%20Component%20Object%20Reference))
  ;[1 0.5992 0.4169 0.4 30] Server
  (Server|MovetoSlot IndexFrom IndexTo ContainerFrom ContainerTo))

(event Custom|Client_AddSlot
  (params (ContainerClass :type Items%20Container%20Component%20Class%20Reference) (Item :type Container%20Item%20Structure))
  ;[0.04772 0.6094 0.2873 0.4 30] Client
  (Default|AddSlot (Default|GetContainerWidget (Utilities|GetMainHud) ContainerClass) Item))

(event Custom|Server_PickupItem
  (params (Item :type Container%20Item%20Structure))
  ;[1 0.5992 0.4169 0.4 30] Server
  (Server|PickupItem Item))

(event Custom|Server_MoveAllItems
  (params (ContainerFrom :type Items%20Container%20Component%20Object%20Reference) (ContainerTo :type Items%20Container%20Component%20Object%20Reference))
  ;[1 0.5992 0.4169 0.4 30] Server
  (Server|MoveAllItems ContainerFrom ContainerTo))

(event Custom|Server_MoveGold
  (params (ContainerFrom :type Items%20Container%20Component%20Object%20Reference) (ContainerTo :type Items%20Container%20Component%20Object%20Reference))
  ;[1 0.5992 0.4169 0.4 30] Server
  (Server|MoveGold ContainerFrom ContainerTo))

(event Custom|InitializeWorldContainer
  (params (ContainerItem :type Array%20of%20Container%20Item%20Structures) (GoldAmount :type Integer))
  (bind _hud (Utilities|GetMainHud))
  (bind _worldcontainer (Variables|/Game/MRPGInventorySystem/UMG/WBP_InventoryHUD.WBP_InventoryHUD_C|GetWorldContainer _hud))
  ;[0.04772 0.6094 0.2873 0.4 30] Client
  (Default|InitializeSlots _worldcontainer ContainerItem)
  (Default|UpdateGold _worldcontainer GoldAmount))

(event Custom|Server_RemoveSlot
  (params (ContainerClass :type Items%20Container%20Component%20Object%20Reference) (Index :type Integer))
  ;[1 0.5992 0.4169 0.4 30] Server
  (bind _managers (Server|GetWatchingManagers ContainerClass))
  (for _array_element _managers
    (CallFunction|ClientRemoveSlot _array_element (Utilities|GetClass ContainerClass) Index)))

(event EventTick
  (params (DeltaSeconds :type Float%20%28single-precision%29))
  ;[1 0.5992 0.4169 0.4] Server - track player and close container when player moves
  (if (>= (Math|Vector|VectorLength (- (Transformation|GetActorLocation (Pawn|GetControlledPawn (.AsPlayer%20Controller (Utilities|Casting|CastToPlayerController (Components|GetOwner))))) (Variables|Default|GetObservePlayerPosition))) 4e+01)
    (bind _asinventory_player_controller (Utilities|Casting|CastToInventoryPlayerController (Components|GetOwner)))
    (if (Variables|Default|GetIsStore)
      (Default|ServerCloseWorldStore _asinventory_player_controller)
      (else
        (Default|ServerCloseContainer _asinventory_player_controller)))))

(fn DragItemBegin
  (params (DraggablePayload :type Draggable%20Payload%20Object%20Reference))
  (Default|CallOnDragItemBegin DraggablePayload))

(fn DragItemEnd
  (Default|CallOnDragItemEnd))

(fn MovetoSlot
  (params (IndexFrom :type Integer) (IndexTo :type Integer) (ContainerFrom :type Items%20Container%20Component%20Object%20Reference) (ContainerTo :type Items%20Container%20Component%20Object%20Reference))
  (LocalVariables|SetSlotFrom (Utilities|Struct|MakeSlotDefinition ContainerFrom IndexFrom))
  (LocalVariables|SetSlotTo (Utilities|Struct|MakeSlotDefinition ContainerTo IndexTo))
  (if (not (Variables|/Game/MRPGInventorySystem/Blueprints/Components/ItemsContainerComponent.ItemsContainerComponent_C|GetIsGlobal ContainerTo)) ; global target container abort
    (if (Variables|/Game/MRPGInventorySystem/Blueprints/Components/ItemsContainerComponent.ItemsContainerComponent_C|GetIsGlobal ContainerFrom)
      (if (== (Utilities|GetClass ContainerTo) "/Game/MRPGInventorySystem/Blueprints/Components/EquipmentComponent.EquipmentComponent_C") ; Global to Equipement only allowed
        (Server|PickupItem (Default|GetInventoryItem (.container (LocalVariables|GetSlotTo)) (.index (LocalVariables|GetSlotTo))))
        (Server|SetItem (.container (LocalVariables|GetSlotTo)) (.index (LocalVariables|GetSlotTo)) (Default|GetInventoryItem (.container (LocalVariables|GetSlotFrom)) (.index (LocalVariables|GetSlotFrom)))))
      (elif (not (Utilities|Equals (LocalVariables|GetSlotFrom) (LocalVariables|GetSlotTo))) ; the same slot abort
        (if (Utilities|SameType (LocalVariables|GetSlotFrom) (LocalVariables|GetSlotTo)) ; consolidate or replace
          (Helper|ConsolidateStackSlots (LocalVariables|GetSlotFrom) (LocalVariables|GetSlotTo))
          (else
            (Helper|ReplaceSlots (LocalVariables|GetSlotFrom) (LocalVariables|GetSlotTo))))))))

(fn ReplaceSlots
  (params (SlotFrom :type Slot%20Definition%20Structure%20%28by%20ref%29) (SlotTo :type Slot%20Definition%20Structure%20%28by%20ref%29))
  (Utilities|CanbeEquiped SlotFrom SlotTo
    (:True
      (Utilities|CanbeEquiped SlotTo SlotFrom
        (:True
          (LocalVariables|SetTempItemFrom (Default|GetInventoryItem (.container SlotFrom) (.index SlotFrom)))
          (Server|SetItem (.container SlotFrom) (.index SlotFrom) (Default|GetInventoryItem (.container SlotTo) (.index SlotTo)))
          (Server|SetItem (.container SlotTo) (.index SlotTo) (LocalVariables|GetTempItemFrom)))))))

(fn ConsolidateStackSlots
  (params (SlotFrom :type Slot%20Definition%20Structure%20%28by%20ref%29) (SlotTo :type Slot%20Definition%20Structure%20%28by%20ref%29))
  (bind _output (Default|GetInventoryItem (.container SlotFrom) (.index SlotFrom)))
  (bind _output_2 (Default|GetInventoryItem (.container SlotTo) (.index SlotTo)))
  (bind (_itemid _quantity) (Utilities|Struct|BreakContainerItem _output))
  (bind _quantity_2 (Utilities|Struct|BreakContainerItem _output_2))
  (bind _itemdata (CallFunction|GetItemData _itemid))
  (bind _returnvalue (+ _quantity _quantity_2))
  (bind _maxquantity (Utilities|Struct|BreakInventoryData _itemdata))
  (bind _structout (Utilities|Struct|SetmembersinContainerItem _output (- _returnvalue _maxquantity)))
  (LocalVariables|SetTempItemFrom _structout)
  (bind _structout_2 (Utilities|Struct|SetmembersinContainerItem _output_2 (Math|Integer|Clamp(Integer) _returnvalue 0 _maxquantity)))
  (LocalVariables|SetTempItemTo _structout_2)
  (if (> (.index SlotFrom) (.index SlotTo))
    (Utilities|FlowControl|Sequence
      (:then_0
        (Server|SetItem (.container SlotFrom) (.index SlotFrom) (LocalVariables|GetTempItemTo) :!label _label))
      (:then_1
        (Server|SetItem (.container SlotTo) (.index SlotTo) (LocalVariables|GetTempItemFrom) :!label _label_2)))
    (else
      (Utilities|FlowControl|Sequence
        (:then_0
          (goto _label_2))
        (:then_1
          (goto _label))))))

(fn SetItem
  (params (Container :type Items%20Container%20Component%20Object%20Reference) (Index :type Integer) (Item :type Container%20Item%20Structure))
  (if (<= (.Quantity (Utilities|Struct|BreakContainerItem Item)) 0)
    (bind _removed (Default|ClearItem Container Index))
    (if _removed
      (CallFunction|ServerRemoveSlot Container Index)
      (else
        (CallFunction|ServerSetSlot Container Index Item :!label _label)))
    (else
      (Default|SetItem Container Index Item)
      (goto _label))))

(fn MovetoContainer
  (params (IndexFrom :type Integer) (ContainerFrom :type Items%20Container%20Component%20Object%20Reference) (ContainerTo :type Items%20Container%20Component%20Object%20Reference))
  (LocalVariables|SetSlotFrom (Utilities|Struct|MakeSlotDefinition ContainerFrom IndexFrom))
  (if (not (or (Variables|/Game/MRPGInventorySystem/Blueprints/Components/ItemsContainerComponent.ItemsContainerComponent_C|GetIsGlobal ContainerFrom) (Variables|/Game/MRPGInventorySystem/Blueprints/Components/ItemsContainerComponent.ItemsContainerComponent_C|GetIsGlobal ContainerTo))) ; ignore global containers
    (if (Variables|/Game/MRPGInventorySystem/Blueprints/Components/ItemsContainerComponent.ItemsContainerComponent_C|GetIsStore ContainerFrom) ; Purchase store item or drag from chest
      (if (!= ContainerFrom ContainerTo)
        ;[1 1 1] Local store
        (bind _paid (Server|TryPayGold (.ShopPurchaseCost (Utilities|Struct|BreakInventoryData (CallFunction|GetItemData (.ItemID (Utilities|Struct|BreakContainerItem (Default|GetInventoryItem (.container (LocalVariables|GetSlotFrom)) (.index (LocalVariables|GetSlotFrom))))))))))
        (if _paid
          (Default|AddItem ContainerTo (Default|GetInventoryItem (.container (LocalVariables|GetSlotFrom)) (.index (LocalVariables|GetSlotFrom))))
          (CallFunction|ServerAddSlot ContainerTo (Default|GetInventoryItem (.container (LocalVariables|GetSlotFrom)) (.index (LocalVariables|GetSlotFrom))))))
      (else
        ;[1 1 1] Storage (chest)
        (Default|AddItem ContainerTo (Default|GetInventoryItem (.container (LocalVariables|GetSlotFrom)) (.index (LocalVariables|GetSlotFrom))))
        (CallFunction|ServerAddSlot ContainerTo (Default|GetInventoryItem (.container (LocalVariables|GetSlotFrom)) (.index (LocalVariables|GetSlotFrom))))
        (Helper|RemoveorClearItem (.container (LocalVariables|GetSlotFrom)) (.index (LocalVariables|GetSlotFrom)))))))

(fn GetWatchingManagers
  (params (ContainerClass :type Items%20Container%20Component%20Object%20Reference))
  (bind _managerslocal (LocalVariables|GetManagersLocal))
  (bind _asstorage_component (Utilities|Casting|CastToStorageComponent ContainerClass)
    (:then
      (for _array_element (Variables|/Game/MRPGInventorySystem/Blueprints/Components/StorageComponent.StorageComponent_C|GetPlayersWatching _asstorage_component)
        (Utilities|Array|Add (LocalVariables|GetManagersLocal) (Variables|/Game/MRPGInventorySystem/Blueprints/InventoryPlayerController.InventoryPlayerController_C|GetInventoryManager _array_element))))
    (:CastFailed
      _))
  (Utilities|Array|AddUnique _managerslocal self)
  (return _managerslocal))

(fn DropItem
  (params (IndexFrom :type Integer) (ContainerFrom :type Items%20Container%20Component%20Object%20Reference))
  (bind _containeritems (Variables|/Game/MRPGInventorySystem/Blueprints/Components/ItemsContainerComponent.ItemsContainerComponent_C|GetContainerItems ContainerFrom))
  (bind _output (Utilities|Array|Get(acopy) _containeritems IndexFrom))
  (if (not (Variables|/Game/MRPGInventorySystem/Blueprints/Components/ItemsContainerComponent.ItemsContainerComponent_C|GetIsGlobal ContainerFrom)) ; Ignore global container
    (if (Utilities|Struct|BreakInventoryData (CallFunction|GetItemData (.ItemID (Utilities|Struct|BreakContainerItem (Default|GetInventoryItem ContainerFrom IndexFrom))))) ; Check if virtual item
      (if (== (Utilities|GetClass ContainerFrom) "/Game/MRPGInventorySystem/Blueprints/Components/EquipmentComponent.EquipmentComponent_C") ; for virtual items just remove them if equiped
        (Helper|RemoveorClearItem ContainerFrom IndexFrom :!label _label))
      (else
        (Game|SpawnActorfromClass "/Game/MRPGInventorySystem/Blueprints/Actors/BP_PickupItem.BP_PickupItem_C" (Math|Conversions|ToTransform(Vector) (Utilities|GetPlayerDropLocation)) "Undefined" 0 0 (.quantity _output) (.itemid _output) 0)
        (goto _label)))))

(fn PickupItem
  (params (Item :type Container%20Item%20Structure))
  (bind _self self)
  (bind _inventory_character (CallFunction|GetOwningCharacter _self))
  (bind _inventorycomponent (Variables|/Game/MRPGInventorySystem/Blueprints/Actors/BP_InventoryCharacter.BP_InventoryCharacter_C|GetInventoryComponent _inventory_character))
  (if (Utilities|Name|NotEqual(Name) (.ItemID (Utilities|Struct|BreakContainerItem Item)) "None")
    (Default|AddItem _inventorycomponent Item)
    (CallFunction|ServerAddSlot _inventorycomponent Item)))

(fn RemoveorClearItem
  (params (Container :type Items%20Container%20Component%20Object%20Reference) (Index :type Integer))
  (bind _removed (Default|ClearItem Container Index))
  (if _removed
    (CallFunction|ServerRemoveSlot Container Index)
    (else
      (CallFunction|ServerSetSlot Container Index (Utilities|Struct|MakeContainerItem "None" -1)))))

(fn MoveAllItems
  (params (ContainerFrom :type Items%20Container%20Component%20Object%20Reference) (ContainerTo :type Items%20Container%20Component%20Object%20Reference))
  (bind _arrayindex (Utilities|Array|ReverseforEachLoop (Variables|/Game/MRPGInventorySystem/Blueprints/Components/ItemsContainerComponent.ItemsContainerComponent_C|GetContainerItems ContainerFrom))
    (:LoopBody
      (Server|MovetoContainer _arrayindex ContainerFrom ContainerTo))))

(fn MoveGold
  (params (ContainerFrom :type Items%20Container%20Component%20Object%20Reference) (ContainerTo :type Items%20Container%20Component%20Object%20Reference))
  (Variables|/Game/MRPGInventorySystem/Blueprints/Components/ItemsContainerComponent.ItemsContainerComponent_C|SetGoldAmount ContainerTo (+ (Variables|/Game/MRPGInventorySystem/Blueprints/Components/ItemsContainerComponent.ItemsContainerComponent_C|GetGoldAmount ContainerTo) (Variables|/Game/MRPGInventorySystem/Blueprints/Components/ItemsContainerComponent.ItemsContainerComponent_C|GetGoldAmount ContainerFrom)))
  (Variables|/Game/MRPGInventorySystem/Blueprints/Components/ItemsContainerComponent.ItemsContainerComponent_C|SetGoldAmount ContainerFrom 0)
  (CallFunction|ServerUpdateGold ContainerFrom)
  (CallFunction|ServerUpdateGold ContainerTo))

(fn PickupGold
  (params (GoldAmount :type Integer))
  (bind _self self)
  (bind _inventory_character (CallFunction|GetOwningCharacter _self))
  (bind _inventorycomponent (Variables|/Game/MRPGInventorySystem/Blueprints/Actors/BP_InventoryCharacter.BP_InventoryCharacter_C|GetInventoryComponent _inventory_character))
  (Default|AddGold _inventorycomponent GoldAmount)
  (CallFunction|ServerUpdateGold _inventorycomponent))

(fn TryPayGold
  (params (GoldAmount :type Integer))
  (bind _self self)
  (bind _inventory_character (CallFunction|GetOwningCharacter _self))
  (bind _inventorycomponent (Variables|/Game/MRPGInventorySystem/Blueprints/Actors/BP_InventoryCharacter.BP_InventoryCharacter_C|GetInventoryComponent _inventory_character))
  (if (>= (Variables|/Game/MRPGInventorySystem/Blueprints/Components/ItemsContainerComponent.ItemsContainerComponent_C|GetGoldAmount _inventorycomponent) GoldAmount)
    (Variables|/Game/MRPGInventorySystem/Blueprints/Components/ItemsContainerComponent.ItemsContainerComponent_C|SetGoldAmount _inventorycomponent (- (Variables|/Game/MRPGInventorySystem/Blueprints/Components/ItemsContainerComponent.ItemsContainerComponent_C|GetGoldAmount _inventorycomponent) GoldAmount))
    (CallFunction|ServerUpdateGold _inventorycomponent)
    (return true)
    (else
      (return false))))