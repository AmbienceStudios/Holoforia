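; Equipment container component that mirrors its slot contents onto the owning BP_InventoryCharacter as equipped items.
; On BeginPlay it calls Equip for every entry in ContainerItems, passing item ID and slot index.
; SetItem calls Equip after the parent stores the item, while ClearItem calls Unequip before the parent clears it, so the ID remains readable.
; GetType returns each slot's type from EquipementData.
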(event EventBeginPlay
  (CallFunction|InitializeEquipement))

(fn GetType
  (params (Index :type Integer))
  (return (Utilities|Array|Get(acopy) (Variables|Properties|GetEquipementData) Index)))

(fn ClearItem
  (params (Index :type Integer))
  (Default|Unequip (.AsBP%20Inventory%20Character (Utilities|Casting|CastToBP_InventoryCharacter (Components|GetOwner))) (.ItemID (Utilities|Struct|BreakContainerItem (Utilities|Array|Get(acopy) (Variables|Default|GetContainerItems) Index))) Index)
  (bind _removed (|CallParentFunction Index))
  (return _removed))

(fn SetItem
  (params (Index :type Integer) (Item :type Container%20Item%20Structure))
  (|CallParentFunction Index Item)
  (bind _asbp_inventory_character (Utilities|Casting|CastToBP_InventoryCharacter (Components|GetOwner)))
  (Default|Equip _asbp_inventory_character (.ItemID (Utilities|Struct|BreakContainerItem (Utilities|Array|Get(acopy) (Variables|Default|GetContainerItems) Index))) Index)
  (return))

(fn InitializeEquipement
  (bind _asbp_inventory_character (Utilities|Casting|CastToBP_InventoryCharacter (Components|GetOwner)))
  (for (_array_element _array_index) (Variables|Default|GetContainerItems)
    (Default|Equip _asbp_inventory_character (Utilities|Struct|BreakContainerItem _array_element) _array_index)))