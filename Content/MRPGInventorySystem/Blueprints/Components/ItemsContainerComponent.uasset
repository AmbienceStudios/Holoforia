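; Actor component for the MRPG inventory system that stores a container's list of items and a gold amount.
; Provides functions to add, read, set and clear items by index, plus add gold, with only AddItem firing the items-change notification.
; Setting an item with zero or lower quantity routes to ClearItem, which removes the entry if removable or otherwise overwrites it with a quantity of -1.
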(fn AddItem
  (params (Item :type Container%20Item%20Structure))
  (Utilities|Array|Add (Variables|Default|GetContainerItems) Item)
  (Default|CallOnItemsChange))

(fn ClearItem
  (params (Index :type Integer))
  (bind _containeritems (Variables|Default|GetContainerItems))
  (if (Variables|Properties|GetisRemovable)
    (Utilities|Array|RemoveIndex _containeritems Index)
    (return true)
    (else
      (Utilities|Array|SetArrayElem _containeritems Index (Utilities|Struct|MakeContainerItem "None" -1))
      (return false))))

(fn GetInventoryItem
  (params (Index :type Integer))
  (return (Utilities|Array|Get(acopy) (Variables|Default|GetContainerItems) Index)))

(fn SetItem
  (params (Index :type Integer) (Item :type Container%20Item%20Structure))
  (if (<= (.Quantity (Utilities|Struct|BreakContainerItem Item)) 0)
    (CallFunction|ClearItem Index) ; REMOVE
    (else
      (Utilities|Array|SetArrayElem (Variables|Default|GetContainerItems) Index Item) ; SET
    ))
  (return))

(fn AddGold
  (params (GoldAmount :type Integer))
  (Variables|Default|SetGoldAmount (+ GoldAmount (Variables|Default|GetGoldAmount))))