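; Selectable world object with a mesh and floating title that responds to mouse hover and click in the inventory system.
; Construction script applies mesh, title and height; cursor events come from the GetMeshForCursorOver component.
; Tick runs only while hovered, turning the title toward the camera and toggling it and the custom-depth outline by player distance through paired DoOnce gates.
; Clicks go to the inventory player controller's server event, without a distance check here.
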(event Custom|StartOverlap
  (bind _staticmeshcomponent (Variables|Default|GetStaticMeshComponent))
  (bind _selectableobjectinfo (Variables|Default|GetSelectableObjectInfo))
  ;[1 1 1] Outline effect enable / disable when mouse is hovered over and distance
  (Utilities|FlowControl|DoOnce false
    (:Completed
      (Utilities|FlowControl|Sequence
        (:then_0
          (Rendering|SetRenderCustomDepth _staticmeshcomponent true)
          (Development|SetHiddeninGame _selectableobjectinfo false false))
        (:then_1
          (Utilities|FlowControl|DoOnce false) ; enters at Reset
        )))))

(event Custom|BeginCursorOver
  (params (TouchedComponent :type Primitive%20Component%20Object%20Reference))
  ;[1 1 1] When cursor is over object
  (Actor|Tick|SetActorTickEnabled true)
  (CallFunction|StartOverlap))

(event Custom|EndCursorOver
  (params (TouchedComponent :type Primitive%20Component%20Object%20Reference))
  ;[1 1 1] When cursor is over object
  (Actor|Tick|SetActorTickEnabled false)
  (CallFunction|EndOverlap))

(event Custom|Clicked
  (params (TouchedComponent :type Primitive%20Component%20Object%20Reference) (ButtonPressed :type Key%20Structure))
  ;[1 1 1] Pressing functionality - clients clicked on the object
  (bind _asbp_selectable_object (Utilities|Casting|CastToBP_SelectableObject (Components|GetOwner TouchedComponent)))
  (Default|ServeronSelectableObjectClicked (CallFunction|GetInventoryPlayerController) _asbp_selectable_object))

(event Custom|EndOverlap
  (bind _staticmeshcomponent (Variables|Default|GetStaticMeshComponent))
  (bind _selectableobjectinfo (Variables|Default|GetSelectableObjectInfo))
  ;[1 1 1] Outline effect enable / disable when mouse is hovered over and distance
  (Utilities|FlowControl|DoOnce false
    (:Completed
      (Utilities|FlowControl|Sequence
        (:then_0
          (Rendering|SetRenderCustomDepth _staticmeshcomponent false)
          (Development|SetHiddeninGame _selectableobjectinfo true false))
        (:then_1
          (Utilities|FlowControl|DoOnce false) ; enters at Reset
        )))))

(event EventTick
  (params (DeltaSeconds :type Float%20%28single-precision%29))
  ;[1 1 1] Checks distance to hovered object
  (if (<= (Transformation|GetDistanceTo (Game|Player|GetPlayerPawn 0) self) (Variables|Default|GetMinimalDistanceToObject))
    (CallFunction|RotateTextTowardsPlayer)
    (CallFunction|StartOverlap)
    (else
      (CallFunction|EndOverlap))))

(event EventBeginPlay
  (bind _meshcomponent (CallFunction|GetMeshforCursorOver))
  (EventDispatchers|AssignOnBeginCursorOver _meshcomponent (delegate Custom|BeginCursorOver))
  (EventDispatchers|AssignOnEndCursorOver _meshcomponent (delegate Custom|EndCursorOver))
  (EventDispatchers|AssignOnClicked _meshcomponent (delegate Custom|Clicked)))

(fn ConstructionScript
  (|CallParentFunction)
  (Rendering|Components|TextRender|SetText (Variables|Default|GetSelectableObjectInfo) (Variables|Default|GetTitle))
  (Transformation|SetRelativeLocation (Variables|Default|GetSelectableObjectInfo) (Math|Vector|MakeVector 0.0 0.0 (Variables|Default|GetTitleHeight)) false false)
  (Components|StaticMesh|SetStaticMesh (Variables|Default|GetStaticMeshComponent) (Variables|Default|GetStaticMesh)))

(fn RotateTextTowardsPlayer
  (Transformation|SetWorldRotation (Variables|Default|GetSelectableObjectInfo) (Math|Rotator|FindLookatRotation (Transformation|GetActorLocation) (Transformation|GetActorLocation (Game|GetPlayerCameraManager 0))) false false))

(fn GetMeshforCursorOver
  (return (Variables|Default|GetStaticMeshComponent)))