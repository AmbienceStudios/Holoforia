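; BP_PickupItem is an inventory pickup actor that represents an item, identified by ItemID and Quantity, placed in the world.
; Its construction script looks up the item data by ID to set the static mesh and the selectable object's info text from the item title.
; GetItem packs the ID and quantity into a container item struct for the caller.
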(fn ConstructionScript
  (bind _itemid (Variables|StaticMesh|GetItemID))
  (bind _itemdata (CallFunction|GetItemData _itemid))
  (|CallParentFunction)
  (Components|StaticMesh|SetStaticMesh (Variables|Default|GetStaticMeshComponent) (.staticmesh _itemdata))
  (Rendering|Components|TextRender|SetText (Variables|Default|GetSelectableObjectInfo) (.title _itemdata)))

(fn GetItem
  (return (Utilities|Struct|MakeContainerItem (Variables|StaticMesh|GetItemID) (Variables|StaticMesh|GetQuantity))))