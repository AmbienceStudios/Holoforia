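; BP_PickupGold is a gold pickup actor in the MRPG inventory system, configurable as either a gold bar or a gold coin.
; After running its parent's construction script, it uses the PickupGoldType value to select the title, static mesh, selectable-object label and gold amount.
; The file holds only this setup, with no collection logic of its own.
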(fn ConstructionScript
  (bind _pickupgoldtype (Variables|StaticMesh|GetPickupGoldType))
  (bind _returnvalue (Utilities|Select :Index _pickupgoldtype :NewEnumerator0 "Gold Bar (+5 gold)" :NewEnumerator1 "Gold Coin (+1 gold)"))
  (|CallParentFunction)
  (Variables|Default|SetTitle _returnvalue)
  (Components|StaticMesh|SetStaticMesh (Variables|Default|GetStaticMeshComponent) (Utilities|Select :Index _pickupgoldtype :NewEnumerator0 "/Game/MRPGInventorySystem/Assets/Meshes/SM_GoldBar.SM_GoldBar" :NewEnumerator1 "/Game/MRPGInventorySystem/Assets/Meshes/SM_Coin.SM_Coin"))
  (Rendering|Components|TextRender|SetText (Variables|Default|GetSelectableObjectInfo) _returnvalue)
  (Variables|StaticMesh|SetGoldAmount (Utilities|Select :Index _pickupgoldtype :NewEnumerator0 5 :NewEnumerator1 1)))